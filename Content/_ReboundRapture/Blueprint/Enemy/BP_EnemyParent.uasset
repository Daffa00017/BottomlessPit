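; Base enemy Blueprint that relays state changes to its animation components.
; On BeginPlay it binds to AI move state changes and forwards each new state to the BodyAnim anim instance as a message.
; A separate enemy-mode event stores the state and switches the Sprite flipbook between idle and walk.
; The fire-once and overlap events are empty, as is the construction script.
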(event `self.ReceiveBeginPlay`
  (add `self.OnAIMoveStateChanged` (`|CreateDelegate` :!event `OnAIMoveStateChanged_Event`)))

(event `AI_FireOnce`)

(event `/Game/_ReboundRapture/Blueprint/Interface/BPI_Enemy.I_E1_SetEnemyMode`
  (params (NewState :type "EEnemyMode Enum" :default "Idle"))
  (bind _output_get (set `self.e_EnemyState` NewState))
  (if (`|EnumEquality` _output_get "Idle")
    (`PaperFlipbookComponent.SetFlipbook` (`self.Sprite`) "/Game/_ReboundRapture/Placeholder/Chara/Flipbook/Idle/Ph_Idle.Ph_Idle")
    (else
      (`PaperFlipbookComponent.SetFlipbook` (`self.Sprite`) "/Game/_ReboundRapture/Placeholder/Chara/Flipbook/Walk/Ph_Walk.Ph_Walk"))))

(event `OnAIMoveStateChanged_Event` :!signature `self.OnAIMoveStateChanged`
  (params (Old :type "EAIMovementState Enum" :default "Idle") (New :type "EAIMovementState Enum" :default "Idle"))
  (message `/Game/_ReboundRapture/Blueprint/Interface/BPI_CharacterAnimation.I_E_SetAIMovState` (`PaperZDAnimationComponent.AnimInstance` (`self.BodyAnim`)) New))

(fn `UserConstructionScript`)