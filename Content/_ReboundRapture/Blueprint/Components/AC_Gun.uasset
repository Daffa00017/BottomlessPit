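; Actor component that gives its owner a gun and drives its shooting.
; Setup async-loads the BP_Gun class, spawns it and snaps it to a given parent component socket.
; Start and stop events call StartFire and StopFire, with start also calling an event dispatcher.
; FireEvent sends an interface shoot message to the spawned gun and broadcasts a firing update.
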(event `SetupGunComponent`
  (params (Parent :type "SceneComponent Object Reference") (InputPin :type Name))
  (bind _class (`|LoadAssetClass` "/Game/_ReboundRapture/Blueprint/Gun/BP_Gun.BP_Gun_C")
    (:`Completed`
      (bind _asactor (castclass `Actor` _class))
      (bind _returnvalue (`|SpawnActorFromClass` _asactor (`KismetMathLibrary.MakeTransform` (0.0 0.0 0.0)) "Undefined" "MultiplyWithRoot" null null))
      (bind _output_get (set `self.BP_GunRef` _returnvalue))
      (`Actor.K2_AttachToComponent` _output_get Parent InputPin "SnapToTarget" "SnapToTarget" "KeepRelative" true))))

(event `StartShoot`
  (`self.StartFire`)
  (`self.ED_StartFire`))

(event `StopShoot`
  (`self.StopFire`))

(event `self.FireEvent`
  (message `/Game/_ReboundRapture/Blueprint/Interface/BPI_Gun.I_Shoot` (`self.BP_GunRef`))
  (`self.ED_OnFiringUpdate`))