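; Player character Blueprint for a 2D flipbook game, with separately animated body and arm and a socket-mounted gun.
; Movement and input delegates feed both anim instances and start or stop GunComponent fire; dash, slide-roll and aim starts only print.
; Landing and air-jump spin overrides hide the gun, while arm sort priority changes between ground and air.
; GetTargetLocation projects the mouse onto the character's Y plane.
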(event `self.ReceiveBeginPlay`
  (`self.BindEvent`)
  (`self.SetupBeginPlay`))

(event `self.CustomEventOnLanded`
  (params (HitResult :type "HitResult Structure"))
  ; JumpEvent
  (message `/Game/_ReboundRapture/Blueprint/Interface/BPI_CharacterAnimation.I_SetFallingOfLedge` (`self.AnimInstanceRef`) false)
  (message `/Game/_ReboundRapture/Blueprint/Interface/BPI_CharacterAnimation.I_SetFallingOfLedge` (`self.ArmAnimInstanceRef`) false)
  (`PrimitiveComponent.SetTranslucentSortPriority` (`self.ArmFlipbook`) 5)
  (`PaperZDPlaySlotOverrideAction.PlayAnimationOverrideWithCallbacks` (`self.ArmAnimInstanceRef`) "/Game/_ReboundRapture/Blueprint/Player/Animation/Arm/AnimSequences/ArmLand.ArmLand"
    (:`then`
      (`self.SetActorHiddenInGame` (`/Game/_ReboundRapture/Blueprint/Components/AC_Gun.BP_GunRef` (`self.GunComponent`)) true))))

(event `self.OnWalkingOffLedge`
  (params (PreviousFloorImpactNormal :type "Vector Structure (by ref)") (PreviousFloorContactNormal :type "Vector Structure (by ref)") (PreviousLocation :type "Vector Structure (by ref)") (TimeDelta :type "Float (single-precision)"))
  ; JumpEvent
  (message `/Game/_ReboundRapture/Blueprint/Interface/BPI_CharacterAnimation.I_SetFallingOfLedge` (`self.AnimInstanceRef`) true)
  (message `/Game/_ReboundRapture/Blueprint/Interface/BPI_CharacterAnimation.I_SetFallingOfLedge` (`self.ArmAnimInstanceRef`) true)
  (`PrimitiveComponent.SetTranslucentSortPriority` (`self.ArmFlipbook`) 3)
  (`self.ChangeMovementState` "Jump"))

(event `OnMoveAxisUpdatedDelegate_Event`
  (params (Axis :type "Float (single-precision)") (SpeedX :type "Float (single-precision)"))
  ; movement
  (message `/Game/_ReboundRapture/Blueprint/Interface/BPI_CharacterAnimation.I_SetMoveAxis` (`self.AnimInstanceRef`) (* Axis (`KismetMathLibrary.SelectFloat` -1.0 1.0 (`self.bLookingBack`)))))

(event `OnMovementStateChanged_Event`
  (params (OldState :type "EE_PlayerMovementState Enum" :default "Idle") (NewState :type "EE_PlayerMovementState Enum" :default "Idle"))
  ; movement
  (message `/Game/_ReboundRapture/Blueprint/Interface/BPI_CharacterAnimation.I_SetMovementState` (`self.AnimInstanceRef`) NewState)
  (message `/Game/_ReboundRapture/Blueprint/Interface/BPI_CharacterAnimation.I_SetMovementState` (`self.ArmAnimInstanceRef`) NewState)
  (`KismetSystemLibrary.PrintString` (`|GetEnumeratorNameAsString` NewState)))

(event `OnDashStartedEvent_Event`
  (params (Value :type "Float (single-precision)"))
  ; InputEvent
  (`KismetSystemLibrary.PrintString` (`KismetStringLibrary.Concat_StrStr` "Dash" (`KismetStringLibrary.Conv_DoubleToString` Value))))

(event `OnDashCompletedEvent_Event`
  ; InputEvent
)

(event `OnJumpStartedEvent_Event`
  (params (Value :type "Float (single-precision)"))
  ; InputEvent
  (`PrimitiveComponent.SetTranslucentSortPriority` (`self.ArmFlipbook`) 3)
  (`self.SetActorHiddenInGame` (`/Game/_ReboundRapture/Blueprint/Components/AC_Gun.BP_GunRef` (`self.GunComponent`)) false)
  (if (not (`NavMovementComponent.IsMovingOnGround` (`self.CharacterMovement`)))
    (`PaperZDPlaySlotOverrideAction.PlayAnimationOverrideWithCallbacks` (`self.AnimInstanceRef`) "/Game/_ReboundRapture/Blueprint/Player/Animation/AnimSequences/Ph_AirSpin.Ph_AirSpin" "DefaultSlot" 1.2
      (:`then`
        (`self.SetActorHiddenInGame` (`/Game/_ReboundRapture/Blueprint/Components/AC_Gun.BP_GunRef` (`self.GunComponent`)) true)
        (`PaperZDAnimInstance.JumpToNode` (`self.ArmAnimInstanceRef`) "JumpEmpty" "ArmLocomotion"))
      (:`OnCompleted`
        (`self.SetActorHiddenInGame` (`/Game/_ReboundRapture/Blueprint/Components/AC_Gun.BP_GunRef` (`self.GunComponent`)) false)
        (`PaperZDAnimInstance.JumpToNode` (`self.ArmAnimInstanceRef`) "JumpIdle" "ArmLocomotion")))))

(event `OnJumpCompletedEvent_Event`
  ; InputEvent
)

(event `OnShootStartedEvent_Event`
  (params (Value :type "Float (single-precision)"))
  ; InputEvent
  (`/Game/_ReboundRapture/Blueprint/Components/AC_Gun.StartShoot` (`self.GunComponent`)))

(event `OnShootCompletedEvent_Event`
  ; InputEvent
  (`/Game/_ReboundRapture/Blueprint/Components/AC_Gun.StopShoot` (`self.GunComponent`)))

(event `OnSlideRollStartedEvent_Event`
  (params (Value :type "Float (single-precision)"))
  ; InputEvent
  (`KismetSystemLibrary.PrintString` (`KismetStringLibrary.Concat_StrStr` "SlideRoll" (`KismetStringLibrary.Conv_DoubleToString` Value))))

(event `OnSlideRollCompletedEvent_Event`
  ; InputEvent
)

(event `OnAimStartedEvent_Event`
  (params (Value :type "Float (single-precision)"))
  ; InputEvent
  (`KismetSystemLibrary.PrintString` (`KismetStringLibrary.Concat_StrStr` "Aim" (`KismetStringLibrary.Conv_DoubleToString` Value))))

(event `OnAimCompletedEvent_Event`
  ; InputEvent
)

(event `/Game/_ReboundRapture/Blueprint/Interface/BPI_Player.I_P1_HideGunWhenLanding`
  (params (`True?` :type Boolean))
  ; InputEvent
  (switch `EE_PlayerMovementState` (`self.CurrentMovementState`)
    (:`Idle`
      _)
    (:`Walk`
      (`KismetSystemLibrary.Delay` 0.1)))
  (`self.SetActorHiddenInGame` (`/Game/_ReboundRapture/Blueprint/Components/AC_Gun.BP_GunRef` (`self.GunComponent`)) `True?`))

(event `StartWallSlide`)

(fn `BindEvent`
  (add `self.OnMoveAxisUpdatedDelegate` (`|CreateDelegate` :!event `OnMoveAxisUpdatedDelegate_Event`))
  (add `self.OnMovementStateChanged` (`|CreateDelegate` :!event `OnMovementStateChanged_Event`))
  (add `self.OnDashStartedEvent` (`|CreateDelegate` :!event `OnDashStartedEvent_Event`))
  (add `self.OnDashCompletedEvent` (`|CreateDelegate` :!event `OnDashCompletedEvent_Event`))
  (add `self.OnJumpStartedEvent` (`|CreateDelegate` :!event `OnJumpStartedEvent_Event`))
  (add `self.OnJumpCompletedEvent` (`|CreateDelegate` :!event `OnJumpCompletedEvent_Event`))
  (add `self.OnShootStartedEvent` (`|CreateDelegate` :!event `OnShootStartedEvent_Event`))
  (add `self.OnShootCompletedEvent` (`|CreateDelegate` :!event `OnShootCompletedEvent_Event`))
  (add `self.OnSlideRollStartedEvent` (`|CreateDelegate` :!event `OnSlideRollStartedEvent_Event`))
  (add `self.OnSlideRollCompletedEvent` (`|CreateDelegate` :!event `OnSlideRollCompletedEvent_Event`))
  (add `self.OnAimStartedEvent` (`|CreateDelegate` :!event `OnAimStartedEvent_Event`))
  (add `self.OnAimCompletedEvent` (`|CreateDelegate` :!event `OnAimCompletedEvent_Event`)))

(fn `GetTargetLocation`
  (returns (ReturnValue :type Boolean) (TargetLocation :type "Vector Structure"))
  (bind (_returnvalue_x _returnvalue_y) (`KismetMathLibrary.BreakVector` (`self.K2_GetActorLocation`)))
  (bind (_worldlocation _worlddirection _returnvalue) (`PlayerController.DeprojectMousePositionToWorld` (`GameplayStatics.GetPlayerController` 0)))
  (bind _y (.y _worlddirection))
  (bind _returnvalue_2 (- _returnvalue_y (.y _worldlocation)))
  (if _returnvalue
    (return _returnvalue (+ _worldlocation (* _worlddirection (`KismetMathLibrary.SelectFloat` _returnvalue_2 (/ _returnvalue_2 _y) (== _y 0.0)))))
    (else
      (return false (0.0 0.0 0.0)))))

(fn `I_P1_GetPlayerRef`
  (returns (Ref :type "Object Object Reference"))
  (return null))

(fn `SetupBeginPlay`
  (bind _animinstanceref (`self.AnimInstanceRef`))
  (set `self.AnimInstanceRef` (`PaperZDAnimationComponent.AnimInstance` (`self.AnimationComponent`)))
  (message `/Game/_ReboundRapture/Blueprint/Interface/BPI_CharacterAnimation.I_SetPlayerAnim` _animinstanceref "RR_Placeholder")
  (message `/Game/_ReboundRapture/Blueprint/Interface/BPI_CharacterAnimation.I_UseMoveAxis` _animinstanceref true)
  (set `self.ArmAnimInstanceRef` (`PaperZDAnimationComponent.AnimInstance` (`self.ArmAnim`)))
  (set `self.JumpMaxCount` (`self.MaxJumpCount`))
  (`/Game/_ReboundRapture/Blueprint/Components/AC_Gun.SetupGunComponent` (`self.GunComponent`) (`self.ArmFlipbook`) "GunSocket"))

(fn `UserConstructionScript`)