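; Pooled effects actor that shows one-shot flipbook VFX, including bullet impacts with trails.
; Interface events set the flipbook's color and rotation, then call ActivateVFX with an animation and location; the bullet variant first runs ActivateTrail between impact and muzzle.
; A separate event hands the actor back to the GameMode's pool via an interface message.
; An unconnected chain holds player-facing, delay-then-pool playback logic that never runs.
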(event `self.ReceiveBeginPlay`
  (`PaperFlipbookComponent.SetLooping` (`self.VFXFlipbook`) false))

(event `self.PoolObjectToGameMode`
  (message `/Game/_ReboundRapture/Blueprint/Interface/BPI_GameMode.I_GM_PoolFVX` (`GameplayStatics.GetGameMode`) self))

(event `/Game/_ReboundRapture/Blueprint/Interface/BPI_Actor.I_ActivateTrailAndBulletImpact`
  (params (MuzzleLoc :type "Vector Structure") (ImpactLoc :type "Vector Structure") (Anim :type "PaperFlipbook Object Reference"))
  (bind _vfxflipbook (`self.VFXFlipbook`))
  (`PaperFlipbookComponent.SetSpriteColor` _vfxflipbook (`self.Lc_BulletColor`))
  (`SceneComponent.K2_SetRelativeRotation` :`self` _vfxflipbook)
  (`self.ActivateTrail` ImpactLoc MuzzleLoc)
  (`self.ActivateVFX` Anim ImpactLoc))

(event `/Game/_ReboundRapture/Blueprint/Interface/BPI_Actor.I_ActivateFVX`
  (params (Anim :type "PaperFlipbook Object Reference") (ImpactLoc :type "Vector Structure"))
  (bind _vfxflipbook (`self.VFXFlipbook`))
  (`PaperFlipbookComponent.SetSpriteColor` _vfxflipbook (`self.Lc_OriginColor`))
  (`SceneComponent.K2_SetRelativeRotation` _vfxflipbook (struct :`Pitch` 90.0) false false)
  (`SceneComponent.SetHiddenInGame` (`self.TrailSprite`) false false)
  (`self.ActivateVFX` Anim ImpactLoc))

(fn `UserConstructionScript`)