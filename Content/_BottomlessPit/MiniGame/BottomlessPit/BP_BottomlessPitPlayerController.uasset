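; Player controller for the Bottomless Pit minigame that owns the game's camera.
; On BeginPlay it spawns a DownWell-style lite camera high above the player character and adopts it as the view target with a short blend.
; Interface events for first input, death and restart are forwarded as messages to that camera actor.
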(event `self.ReceiveBeginPlay`
  (bind _returnvalue (`|SpawnActorFromClass` "/Game/_ReboundRapture/Blueprint/Camera/BP_DownWellLiteCam.BP_DownWellLiteCam_C" (`KismetMathLibrary.MakeTransform` (+ (`self.K2_GetActorLocation` (`GameplayStatics.GetPlayerCharacter` 0)) (0.0 0.0 1550.0))) "Undefined" "MultiplyWithRoot" null null))
  (bind _output_get (set `self.Reff_CameraManager` _returnvalue))
  (`CPP_CameraManager.AdoptAsViewTarget` _output_get 0.25))

(event `/Game/_ReboundRapture/Blueprint/Interface/BPI_PlayerController.I_Pc_OnFirstInput`
  (message `/Game/_ReboundRapture/Blueprint/Interface/BPI_Actor.I_Cam_OnFirstInput` (`self.Reff_CameraManager`)))

(event `/Game/_ReboundRapture/Blueprint/Interface/BPI_PlayerController.I_Pc_OnDead`
  (message `/Game/_ReboundRapture/Blueprint/Interface/BPI_Actor.I_Cam_OnDead` (`self.Reff_CameraManager`)))

(event `/Game/_ReboundRapture/Blueprint/Interface/BPI_PlayerController.I_Pc_OnRestart`
  (message `/Game/_ReboundRapture/Blueprint/Interface/BPI_Actor.I_Cam_OnRestart` (`self.Reff_CameraManager`)))

(fn `UserConstructionScript`)