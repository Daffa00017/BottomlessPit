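; Game mode for the Bottomless Pit minigame that pools effect and projectile actors and relays score changes to the HUD.
; Interface events activate pooled actors, spawning new ones when a pool is empty.
; Effects play one of three random flipbook variants, async-loaded from a data table on first use, polled by timer until valid, then cached by name.
; The score start and stop events call the opposite scoring functions.
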(event `self.ReceiveBeginPlay`
  (`self.BindingEvent`)
  (set `self.TrackedActorRef` (`GameplayStatics.GetPlayerCharacter` 0))
  (`KismetSystemLibrary.DelayUntilNextTick`)
  (message `/Game/_ReboundRapture/Blueprint/Interface/BPI_HUDAndUI.I_UI_Blp_UpdateScore` (`PlayerController.GetHUD` (`GameplayStatics.GetPlayerController` 0)) 0.0))

(event `/Game/_ReboundRapture/Blueprint/Interface/BPI_GameMode.I_GM_SpawnFVX`
  (params (PoolSize :type Integer))
  ;[0.836 0.8594 0.3309] VFX Stuff
  (for _ (range (+ PoolSize 1))
    (bind _returnvalue (`|SpawnActorFromClass` "/Game/_ReboundRapture/Blueprint/VFX/BP_Effects.BP_Effects_C" (`KismetMathLibrary.MakeTransform` (0.0 0.0 0.0)) "Undefined" "MultiplyWithRoot" null self null))
    (bind _output_get (set `self.FVXRef` _returnvalue))
    (`KismetArrayLibrary.Array_Add` (`self.FVXPool`) _output_get)))

(event `/Game/_ReboundRapture/Blueprint/Interface/BPI_GameMode.I_GM_PoolFVX`
  (params (Reff :type "Object Object Reference"))
  ;[0.836 0.8594 0.3309] VFX Stuff
  (`KismetArrayLibrary.Array_Add` (`self.FVXPool`) Reff))

(event `CE_AsyncLoadBulletVFX`
  (params (MuzzleLoc :type "Vector Structure") (ImpactLoc :type "Vector Structure") (n_VFXAnimName :type Name))
  ;[0.836 0.8594 0.3309] VFX Stuff
  (set `self.v_MuzzleLoc` MuzzleLoc)
  (set `self.v_ImpactLoc` ImpactLoc)
  (bind _output_get (set `self.n_VFXAnimName` n_VFXAnimName))
  (bind (_rowname _vfx) (`Util_BpAsyncVFXFlipbooks.LoadVFXFlipbooksRowAsync` (`self.DT_VFXAnim`) _output_get)
    (:`OnCompleted`
      (bind _output_get_2 (set `self.s_Fvx` _vfx))
      (bind (_animvar1 _animvar2 _animvar3) (break `VFXAnimationResolved` _output_get_2))
      (set `self.Pf_VFXAnimVar1` _animvar1)
      (set `self.Pf_VFXAnimVar2` _animvar2)
      (set `self.Pf_VFXAnimVar3` _animvar3)
      (bind _returnvalue (`KismetSystemLibrary.K2_SetTimerDelegate` (delegate `Timer_CheckAnimValid`) 0.1 true))
      (set `self.Th_CheckAnim` _returnvalue))))

(event `Timer_CheckAnimValid`
  (bind _s_fvx (`self.s_Fvx`))
  ;[0.836 0.8594 0.3309] VFX Stuff
  (if (and (`KismetSystemLibrary.IsValid` (`self.Pf_VFXAnimVar3`)) (`KismetSystemLibrary.IsValid` (`self.Pf_VFXAnimVar1`)) (`KismetSystemLibrary.IsValid` (`self.Pf_VFXAnimVar2`)))
    (`BlueprintMapLibrary.Map_Add` (`self.FVXAnimPool`) (`self.n_VFXAnimName`) _s_fvx)
    (`self.ActivateBulletFVX` (`self.v_MuzzleLoc`) (`self.v_ImpactLoc`) _s_fvx)
    (`KismetSystemLibrary.K2_ClearAndInvalidateTimerHandle` (`self.Th_CheckAnim`))
    (else
      (`KismetSystemLibrary.PrintString` "AnimStillAsyncLoad"))))

(event `CE_AsyncLoadVFX`
  (params (ImpactLoc :type "Vector Structure") (n_VFXAnimName :type Name))
  ;[0.836 0.8594 0.3309] VFX Stuff
  (set `self.v_ImpactLoc` ImpactLoc)
  (bind _output_get (set `self.n_VFXAnimName` n_VFXAnimName))
  (bind (_rowname _vfx) (`Util_BpAsyncVFXFlipbooks.LoadVFXFlipbooksRowAsync` (`self.DT_VFXAnim`) _output_get)
    (:`OnCompleted`
      (bind _output_get_2 (set `self.s_Fvx` _vfx))
      (bind (_animvar1 _animvar2 _animvar3) (break `VFXAnimationResolved` _output_get_2))
      (set `self.Pf_VFXAnimVar1` _animvar1)
      (set `self.Pf_VFXAnimVar2` _animvar2)
      (set `self.Pf_VFXAnimVar3` _animvar3)
      (bind _returnvalue (`KismetSystemLibrary.K2_SetTimerDelegate` (delegate `CheckTimerVFXValid`) 0.1 true))
      (set `self.Th_CheckAnim` _returnvalue))))

(event `CheckTimerVFXValid`
  (bind _s_fvx (`self.s_Fvx`))
  ;[0.836 0.8594 0.3309] VFX Stuff
  (if (and (`KismetSystemLibrary.IsValid` (`self.Pf_VFXAnimVar3`)) (`KismetSystemLibrary.IsValid` (`self.Pf_VFXAnimVar1`)) (`KismetSystemLibrary.IsValid` (`self.Pf_VFXAnimVar2`)))
    (`BlueprintMapLibrary.Map_Add` (`self.FVXAnimPool`) (`self.n_VFXAnimName`) _s_fvx)
    (`self.ActivateFVX` (`self.v_ImpactLoc`) _s_fvx)
    (`KismetSystemLibrary.K2_ClearAndInvalidateTimerHandle` (`self.Th_CheckAnim`))
    (else
      (`KismetSystemLibrary.PrintString` "AnimStillAsyncLoad"))))

(event `/Game/_ReboundRapture/Blueprint/Interface/BPI_GameMode.I_GM_ActivateTrailAndBulletImpact`
  (params (MuzzleLoc :type "Vector Structure") (ImpactLoc :type "Vector Structure") (AnimName :type Name))
  (bind (_value _returnvalue) (`BlueprintMapLibrary.Map_Find` (`self.FVXAnimPool`) AnimName))
  ;[0.836 0.8594 0.3309] VFX Stuff
  (if _returnvalue
    (`self.ActivateBulletFVX` MuzzleLoc ImpactLoc _value)
    (else
      (`self.CE_AsyncLoadBulletVFX` MuzzleLoc ImpactLoc AnimName))))

(event `/Game/_ReboundRapture/Blueprint/Interface/BPI_GameMode.I_GM_ActivateFVX`
  (params (ImpactLoc :type "Vector Structure") (AnimName :type Name))
  (bind (_value _returnvalue) (`BlueprintMapLibrary.Map_Find` (`self.FVXAnimPool`) AnimName))
  ;[0.836 0.8594 0.3309] VFX Stuff
  (if _returnvalue
    (`self.ActivateFVX` ImpactLoc _value)
    (else
      (`self.CE_AsyncLoadVFX` ImpactLoc AnimName))))

(event `/Game/_ReboundRapture/Blueprint/Interface/BPI_GameMode.I_GM_SpawnProjectile`
  (params (PoolSize :type Integer))
  ;[0.3698 0.0666 0.07019] projectile
  (for _ (range (+ PoolSize 1))
    (bind _returnvalue (`|SpawnActorFromClass` "/Game/_ReboundRapture/Blueprint/Projectile/BP_Projectile.BP_Projectile_C" (`KismetMathLibrary.MakeTransform` (0.0 0.0 0.0)) "Undefined" "MultiplyWithRoot" null self null))
    (bind _output_get (set `self.ProjectileRef` _returnvalue))
    (`KismetArrayLibrary.Array_Add` (`self.ProjectileArray`) _output_get)))

(event `/Game/_ReboundRapture/Blueprint/Interface/BPI_GameMode.I_GM_PoolProjectile`
  (params (Reff :type "Object Object Reference"))
  ;[0.3698 0.0666 0.07019] projectile
  (`KismetArrayLibrary.Array_Add` (`self.ProjectileArray`) Reff))

(event `/Game/_ReboundRapture/Blueprint/Interface/BPI_GameMode.I_GM_ActivateProjectile`
  (params (ProjectileName :type Name) (StartLoc :type "Vector Structure"))
  ;[0.3698 0.0666 0.07019] projectile
  (`self.ActivateProjectile` ProjectileName StartLoc))

(event `/Game/_ReboundRapture/Blueprint/Interface/BPI_GameMode.I_GM_OnFirstInput`)

(event `OnScoreUpdated_Event`
  (params (NewScore :type "Float (single-precision)"))
  (message `/Game/_ReboundRapture/Blueprint/Interface/BPI_HUDAndUI.I_UI_Blp_UpdateScore` (`PlayerController.GetHUD` (`GameplayStatics.GetPlayerController` 0)) NewScore))

(event `/Game/_ReboundRapture/Blueprint/Interface/BPI_GameMode.I_GM_Blp_StopScore`
  (`self.StartScoring`))

(event `/Game/_ReboundRapture/Blueprint/Interface/BPI_GameMode.I_GM_Blp_StartScore`
  (`self.StopScoring`))

(event `/Game/_ReboundRapture/Blueprint/Interface/BPI_GameMode.I_GM_OnRestart`
  (bind _output_get (set `self.PlayerScore` 0.0))
  (message `/Game/_ReboundRapture/Blueprint/Interface/BPI_HUDAndUI.I_UI_Blp_UpdateScore` (`PlayerController.GetHUD` (`GameplayStatics.GetPlayerController` 0)) _output_get))

(fn `ActivateBulletFVX`
  (params (MuzzleLoc :type "Vector Structure") (FVXLoc :type "Vector Structure") (FlipbookAnim :type "VFXAnimationResolved Structure"))
  (locals (AnimToPlay :type "PaperFlipbook Object Reference"))
  (bind (_animvar1 _animvar2 _animvar3) (break `VFXAnimationResolved` FlipbookAnim))
  (bind _output (`|GetArrayItem` (`self.FVXPool`)))
  (set `local.AnimToPlay` (select `int` (`KismetMathLibrary.RandomIntegerInRange` 0 2) :`0` _animvar1 :`1` _animvar2 :`2` _animvar3))
  (`/Engine/EditorBlueprintResources/StandardMacros.IsValid` _output
    (:`Is Valid`
      (message `/Game/_ReboundRapture/Blueprint/Interface/BPI_Actor.I_ActivateTrailAndBulletImpact` _output (`local.MuzzleLoc`) (`local.FVXLoc`) (`local.AnimToPlay`))
      (`KismetArrayLibrary.Array_RemoveItem` (`self.FVXPool`) _output))
    (:`Is Not Valid`
      (bind _returnvalue (`|SpawnActorFromClass` "/Game/_ReboundRapture/Blueprint/VFX/BP_Effects.BP_Effects_C" (`KismetMathLibrary.MakeTransform` (0.0 0.0 0.0)) "Undefined" "MultiplyWithRoot" null self null))
      (message `/Game/_ReboundRapture/Blueprint/Interface/BPI_Actor.I_ActivateTrailAndBulletImpact` _returnvalue (`local.MuzzleLoc`) (`local.FVXLoc`) (`local.AnimToPlay`)))))

(fn `ActivateFVX`
  (params (FVXLoc :type "Vector Structure") (FlipbookAnim :type "VFXAnimationResolved Structure"))
  (locals (AnimToPlay :type "PaperFlipbook Object Reference"))
  (bind (_animvar1 _animvar2 _animvar3) (break `VFXAnimationResolved` FlipbookAnim))
  (bind _output (`|GetArrayItem` (`self.FVXPool`)))
  (set `local.AnimToPlay` (select `int` (`KismetMathLibrary.RandomIntegerInRange` 0 2) :`0` _animvar1 :`1` _animvar2 :`2` _animvar3))
  (`/Engine/EditorBlueprintResources/StandardMacros.IsValid` _output
    (:`Is Valid`
      (message `/Game/_ReboundRapture/Blueprint/Interface/BPI_Actor.I_ActivateFVX` _output (`local.AnimToPlay`) (`local.FVXLoc`))
      (`KismetArrayLibrary.Array_RemoveItem` (`self.FVXPool`) _output))
    (:`Is Not Valid`
      (bind _returnvalue (`|SpawnActorFromClass` "/Game/_ReboundRapture/Blueprint/VFX/BP_Effects.BP_Effects_C" (`KismetMathLibrary.MakeTransform` (0.0 0.0 0.0)) "Undefined" "MultiplyWithRoot" null self null))
      (message `/Game/_ReboundRapture/Blueprint/Interface/BPI_Actor.I_ActivateFVX` _returnvalue (`local.AnimToPlay`) (`local.FVXLoc`)))))

(fn `ActivateProjectile`
  (params (ProjectileName :type Name) (StartLoc :type "Vector Structure"))
  (bind _output (`|GetArrayItem` (`self.ProjectileArray`)))
  (`/Engine/EditorBlueprintResources/StandardMacros.IsValid` _output
    (:`Is Valid`
      (message `/Game/_ReboundRapture/Blueprint/Interface/BPI_Actor.I_ActivateProjectile` _output (`local.ProjectileName`) (`local.StartLoc`))
      (`KismetArrayLibrary.Array_RemoveItem` (`self.ProjectileArray`) _output))
    (:`Is Not Valid`
      (bind _returnvalue (`|SpawnActorFromClass` "/Game/_ReboundRapture/Blueprint/Projectile/BP_Projectile.BP_Projectile_C" (`KismetMathLibrary.MakeTransform` (0.0 0.0 0.0)) "Undefined" "MultiplyWithRoot" null self null))
      (message `/Game/_ReboundRapture/Blueprint/Interface/BPI_Actor.I_ActivateProjectile` _returnvalue (`local.ProjectileName`) (`local.StartLoc`)))))

(fn `BindingEvent`
  (add `self.OnScoreUpdated` (`|CreateDelegate` :!event `OnScoreUpdated_Event`)))

(fn `UserConstructionScript`)