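; Player character for the Bottomless Pit minigame: a falling sprite hero that jumps and fires projectiles downward, tracking ammo.
; Down-smash ramps gravity via timeline and deals radial damage on landing, followed by a jump cooldown.
; Health and hit-impact components handle damage, knockback and death, with timeline-driven mercy-invincibility flashing.
; Interface messages drive HUD, GameMode effects and score, animation and level generator, while any key starts or restarts the run.
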(event OnHealthChange(Health)
  (params (NewHealth :type Float%20%28single-precision%29))
  ;[0.8941 0.2251 0.6132 0.5] Health Event
  (Class|BPIHUDandUI|IUIonHealthChange(Message) (Variables|Default|GetRef_HUD) NewHealth))

(event EDonFiringUpdate(FireComponent)
  (bind _returnvalue (Game|GetGameMode))
  ;[0.15 0.15 0.15 0.5] FireEvent
  (if (|FireProjectileCondition)
    (Class|CPPDownwellLiteCharacter|JumpFunction)
    (if (not (Class|CPPPaperZDParentCharacter|IsGrounded))
      (Class|BPIGameMode|IGMActivateFVX(Message) _returnvalue (CallFunction|GetCapsuleBottomLoc) "BlpPrpjectileSpawn")
      (Class|BPIGameMode|IGMActivateProjectile(Message) _returnvalue "BlpBullet" (- (CallFunction|GetCapsuleBottomLoc) "0.000000,0.000000,20.000000"))
      (Utilities|FlowControl|DelayUntilNextTick)
      (Class|BPIHUDandUI|IUIBlponCurrentAmmoChange(Message) (Variables|Default|GetRef_HUD) (Variables|Default|GetCurrentAmmoCount)))))

(event OnMaxHealthChange(Health)
  (params (NewMaxHealth :type Float%20%28single-precision%29))
  ;[0.8941 0.2251 0.6132 0.5] Health Event
  (Class|BPIHUDandUI|IUIonMaxHealthChange(Message) (Variables|Default|GetRef_HUD) NewMaxHealth))

(event OnDead(Health)
  (bind _charactermovement (Variables|Character|GetCharacterMovement))
  ;[0.8941 0.2251 0.6132 0.5] Health Event
  (if (not (Variables|Default|GetIsDead))
    (Variables|Default|SetIsDead true)
    (Class|BPIPlayerController|IPconDead(Message) (Game|GetPlayerController 0))
    (Class|BPIActor|IBlpDeactivatePlatform(Message) (Variables|Default|GetRef_LevelGenerator) false)
    (Pawn|Components|CharacterMovement|SetMovementMode _charactermovement "MOVE_None" 0)
    (Components|Movement|StopMovementImmediately _charactermovement)))

(event Custom|OnMovementStateChanged_Event
  (params (OldState :type EE_PlayerMovementState%20Enum :default "Idle") (NewState :type EE_PlayerMovementState%20Enum :default "Idle"))
  ;[0.15 0.15 0.15 0.5] Movement
  (Class|BPICharacterAnimation|ISetMovementState(Message) (Variables|/Script/PaperZD.PaperZDAnimationComponent|GetAnimInstance (Variables|Default|GetAnimationComponent)) NewState))

(event Custom|OnMoveAxisUpdatedDelegate_Event
  (params (Axis :type Float%20%28single-precision%29) (SpeedX :type Float%20%28single-precision%29))
  ;[0.15 0.15 0.15 0.5] Input
)

(event Custom|StartMercySpriteInvicible
  ;[0.8941 0.2251 0.6132 0.5] Health Event
  (|MercyInvicibleEvent))

(event Custom|OnDashStartedEvent_Event
  (params (Value :type Float%20%28single-precision%29))
  ;[0.15 0.15 0.15 0.5] Input
)

(event Custom|OnDashCompletedEvent_Event
  ;[0.15 0.15 0.15 0.5] Input
)

(event Custom|OnJumpStartedEvent_Event
  (params (Value :type Float%20%28single-precision%29))
  ;[0.15 0.15 0.15 0.5] Input
  (if (not (Variables|Default|GetIsDead))
    (Default|StartShoot (Variables|Default|GetFire%20Component))))

(event Custom|OnJumpCompletedEvent_Event
  ;[0.15 0.15 0.15 0.5] Input
  (Default|StopShoot (Variables|Default|GetFire%20Component)))

(event Custom|OnDownSmashStartedEvent_Event
  (params (Value :type Float%20%28single-precision%29))
  ;[0.15 0.15 0.15 0.5] Input
  (Development|PrintString "SmashDown" true true "(R=1.000000,G=0.104443,B=0.000000,A=1.000000)")
  (if (Variables|Default|GetIsUpdatingGravity)
    (Variables|/Script/Engine.CharacterMovementComponent|SetGravityScale (Variables|Character|GetCharacterMovement) (* (Variables|Default|GetOriGravityScale) 1e+01))
    (else
      (|UpdateGravitySmashDown))))

(event Custom|OnDownSmashCompletedEvent_Event
  ;[0.15 0.15 0.15 0.5] Input
)

(event Custom|ClearCDCanJump
  ;[0.15 0.15 0.15 0.5] Movement
  (Variables|Default|Setb_CanJump true))

(event Custom|FallingDownAnim
  (bind _v_spriteoriginalloc (Variables|Default|Getv_SpriteOriginalLoc))
  (bind _curvalue (|DOVector3D "" 1.5 (+ _v_spriteoriginalloc "0.000000,0.000000,1500.000000") _v_spriteoriginalloc "Linear" false)
    (:OnUpdate
      (Transformation|SetRelativeLocation (Variables|Default|GetSprite) _curvalue false false))))

(event EventBeginPlay
  ;[0.15 0.15 0.15 0.5] Actor Event
  (CallFunction|BindEvent)
  (CallFunction|SetupBeginplay)
  (CallFunction|FallingDownAnim)
  (Default|ChraInitHitImpactComponent (Variables|Default|GetAC_HitImpact) self))

(event Collision|EventActorBeginOverlap
  (params (OtherActor :type Actor%20Object%20Reference))
  ;[0.15 0.15 0.15 0.5] Actor Event
)

(event EventTick
  (params (DeltaSeconds :type Float%20%28single-precision%29))
  ;[0.15 0.15 0.15 0.5] Actor Event
)

(event EventIP1BlpRegisterLaneLevel
  (params (Ref :type Actor%20Object%20Reference))
  ;[0.15 0.15 0.15 0.5] Interface
  (Variables|Default|SetRef_LevelGenerator Ref))

(event EventCustomEventonLanded
  (params (HitResult :type Hit%20Result%20Structure))
  ;[0.15 0.15 0.15 0.5] Movement
  (Class|BPIGameMode|IGMBlpStopScore(Message) (Game|GetGameMode))
  (Class|BPICharacterAnimation|ISetFallingOfLedge(Message) (Variables|Default|GetAnimReff) false)
  (Audio|Components|Audio|Stop (Variables|Default|GetTL_SmashingDownGravity))
  (CallFunction|SmashingDown)
  (Class|BPIHUDandUI|IUIBlponCurrentAmmoChange(Message) (Variables|Default|GetRef_HUD) (Variables|Default|GetCurrentAmmoCount)))

(event EventOnWalkingOffLedge
  (params (PreviousFloorImpactNormal :type Vector%20%28by%20ref%29 :default "0, 0, 0") (PreviousFloorContactNormal :type Vector%20%28by%20ref%29 :default "0, 0, 0") (PreviousLocation :type Vector%20%28by%20ref%29 :default "0, 0, 0") (TimeDelta :type Float%20%28single-precision%29))
  ;[0.15 0.15 0.15 0.5] Movement
  (Class|BPICharacterAnimation|ISetFallingOfLedge(Message) (Variables|Default|GetAnimReff) true))

(event Game|Damage|EventAnyDamage
  (params (Damage :type Float%20%28single-precision%29) (DamageType :type Damage%20Type%20Object%20Reference) (InstigatedBy :type Controller%20Object%20Reference) (DamageCauser :type Actor%20Object%20Reference))
  ;[0.8941 0.2251 0.6132 0.5] Health Event
  (|CheckIfHasMercy)
  (Class|HealthComponent|AddHealth (Variables|Default|GetHealth) (* Damage -1.0))
  (Utilities|IsValid DamageCauser
    (:Is%20Valid
      (Default|ChraRegularKnockBack (Variables|Default|GetAC_HitImpact) 8e+02 4e+02 DamageCauser))))

(event EventIP1PlayGameOverSequence
  ;[0.8941 0.2251 0.6132 0.5] Health Event
  (Class|BPIGameMode|IGMActivateFVX(Message) (Game|GetGameMode) (- (Transformation|GetActorLocation (Game|GetPlayerCharacter 0)) "0.000000,0.000000,5.000000") "BlpGameOver")
  (Utilities|AbpJumptoNode "JumpDeath")
  (Utilities|FlowControl|Delay 1.0)
  (Class|BPIHUDandUI|IUIonDeath(Message) (Variables|Default|GetRef_HUD)))

(event EventIP1ReadytoRestart
  (params (True? :type Boolean))
  ;[0.15 0.15 0.15 0.5] Interface
  (Variables|Default|Setb_IsReadyToRestart True?))

(event EventIP1ApplyAttackStat
  (params (AttackStat :type S%20Attack%20Stat%20Structure))
  ;[0.15 0.15 0.15 0.5] Interface
  (Default|ApplyStatAttack (Variables|Default|GetAC_HitImpact) AttackStat))

(event Input|KeyboardEvents|DebugKeyZ
  (params (Key :type Key%20Structure) (ActionValue :type Input%20Action%20Value%20Structure))
  ;[0.15 0.15 0.15 0.5] Input
  (:Pressed
    (Game|Damage|ApplyDamage self 1.0 0 0)))

(event Input|KeyboardEvents|AnyKey
  (params (Key :type Key%20Structure))
  ;[0.15 0.15 0.15 0.5] Input
  (:Pressed
    (if (Variables|Default|GetIsDead)
      (|Restart)
      (else
        (|MainMenu)))))

(fn ConstructionScript)

(fn BindEvent
  (EventDispatchers|BindEventtoOnMoveAxisUpdatedDelegate (EventDispatchers|CreateEvent :!event Custom|OnMoveAxisUpdatedDelegate_Event))
  (EventDispatchers|BindEventtoOnMovementStateChanged (EventDispatchers|CreateEvent :!event Custom|OnMovementStateChanged_Event))
  (EventDispatchers|BindEventtoOnDashStartedEvent (EventDispatchers|CreateEvent :!event Custom|OnDashStartedEvent_Event))
  (EventDispatchers|BindEventtoOnDashCompletedEvent (EventDispatchers|CreateEvent :!event Custom|OnDashCompletedEvent_Event))
  (EventDispatchers|BindEventtoOnJumpStartedEvent (EventDispatchers|CreateEvent :!event Custom|OnJumpStartedEvent_Event))
  (EventDispatchers|BindEventtoOnJumpCompletedEvent (EventDispatchers|CreateEvent :!event Custom|OnJumpCompletedEvent_Event))
  (EventDispatchers|BindEventtoOnDownSmashStartedEvent (EventDispatchers|CreateEvent :!event Custom|OnDownSmashStartedEvent_Event))
  (EventDispatchers|BindEventtoOnDownSmashCompletedEvent (EventDispatchers|CreateEvent :!event Custom|OnDownSmashCompletedEvent_Event)))

(fn SetupBeginplay
  (bind _maxammocount (Variables|Default|GetMaxAmmoCount))
  (bind _health (Variables|Default|GetHealth))
  (bind _returnvalue (Class|HealthComponent|GetMaxHealth _health))
  (Variables|Default|SetIsDead false)
  (Variables|Default|Setv_SpriteOriginalLoc (Variables|/Script/Engine.SceneComponent|GetRelativeLocation (Variables|Default|GetSprite)))
  (Variables|Default|Setv_PLayerOriginLoc (Transformation|GetActorLocation))
  (Variables|Default|SetRef_HUD (HUD|GetHUD (Game|GetPlayerController 0)))
  (Class|HealthComponent|SetCurrentHealth _health _returnvalue)
  (Class|BPIHUDandUI|IUIonMaxHealthChange(Message) (Variables|Default|GetRef_HUD) _returnvalue)
  (Variables|Default|SetLcs_SpriteOGColor (Class|PaperFlipbookComponent|GetSpriteColor (Variables|Default|GetSprite)))
  (bind _output_get (Variables|Default|SetAnimReff (Variables|/Script/PaperZD.PaperZDAnimationComponent|GetAnimInstance (Variables|Default|GetAnimationComponent))))
  (Class|BPICharacterAnimation|ISetFallingOfLedge(Message) _output_get true)
  (Class|PaperZDAnimInstance|JumptoNode (Variables|Default|GetAnimReff) "Jump_Idle" "Locomotion")
  (Class|BPICharacterAnimation|ISetPlayerAnim(Message) (Variables|Default|GetAnimReff) "Dw_Placeholder")
  (Class|BPICharacterAnimation|IUseMoveAxis(Message) (Variables|Default|GetAnimReff) false)
  (Variables|Default|SetJumpMaxCount (+ (Variables|Default|GetMaxAmmoCount) 1))
  (Variables|Default|SetCurrentAmmoCount _maxammocount)
  (Class|BPIHUDandUI|IUIBlponMaxAmmoChange(Message) (Variables|Default|GetRef_HUD) _maxammocount)
  (Pawn|Components|CharacterMovement|SetMovementMode (Variables|Character|GetCharacterMovement) "MOVE_Falling" 0))

(fn SmashingDown
  (bind _returnvalue (CallFunction|GetCapsuleBottomLoc))
  (bind _self self)
  (if (Variables|Default|GetIsSmashingDown)
    (Variables|Default|Setb_CanJump false)
    (Collision|MultiSphereTraceByChannel _returnvalue _returnvalue 1e+02 "TraceTypeQuery3" false 0 "ForDuration" true "(R=1.000000,G=0.000000,B=0.000000,A=1.000000)" "(R=0.000000,G=1.000000,B=0.000000,A=1.000000)" 1.0)
    (Variables|Default|SetIsSmashingDown false)
    (Class|BPIGameMode|IGMActivateFVX(Message) (Game|GetGameMode) (CallFunction|GetCapsuleBottomLoc) "SlamSmoke")
    (Utilities|Time|SetTimerbyEvent (EventDispatchers|CreateEvent :!event Custom|ClearCDCanJump) (Variables|Default|Getf_JumpCdAfterSmash))
    (Game|Damage|ApplyRadialDamage 1.0 (CallFunction|GetCapsuleBottomLoc) 1e+02 0 (Utilities|Array|MakeArray _self) _self 0 true "ECC_Visibility")
    (else
      (Class|BPIGameMode|IGMActivateFVX(Message) (Game|GetGameMode) (CallFunction|GetCapsuleBottomLoc) "LandSmoke"))))

(fn GetCapsuleBottomLoc
  (bind _returnvalue (Transformation|GetActorLocation))
  (return (Math|Vector|MakeVector (.x _returnvalue) (.y _returnvalue) (- (.z _returnvalue) (Components|Capsule|GetScaledCapsuleHalfHeight (Variables|Default|GetCapsuleComponent))))))

(fn RestartBeginplay
  (bind _returnvalue (Transformation|GetActorLocation))
  (bind _maxammocount (Variables|Default|GetMaxAmmoCount))
  (bind _health (Variables|Default|GetHealth))
  (bind _returnvalue_2 (Class|HealthComponent|GetMaxHealth _health))
  (Pawn|Components|CharacterMovement|SetMovementMode (Variables|Character|GetCharacterMovement) "MOVE_Falling" 0)
  (Variables|Default|SetIsDead false)
  (Transformation|SetActorLocation (Math|Vector|MakeVector (.x (Variables|Default|Getv_PLayerOriginLoc)) (.y _returnvalue) (.z _returnvalue)) false false)
  (Class|HealthComponent|SetCurrentHealth _health _returnvalue_2)
  (Class|BPIHUDandUI|IUIonMaxHealthChange(Message) (Variables|Default|GetRef_HUD) _returnvalue_2)
  (Class|BPICharacterAnimation|ISetFallingOfLedge(Message) (Variables|Default|GetAnimReff) true)
  (Class|BPICharacterAnimation|IUseMoveAxis(Message) (Variables|Default|GetAnimReff) false)
  (Variables|Default|SetJumpMaxCount (+ (Variables|Default|GetMaxAmmoCount) 1))
  (Variables|Default|SetCurrentAmmoCount _maxammocount)
  (Class|BPIHUDandUI|IUIBlponMaxAmmoChange(Message) (Variables|Default|GetRef_HUD) _maxammocount))

(fn IP1GetPlayerRef
  (return self))