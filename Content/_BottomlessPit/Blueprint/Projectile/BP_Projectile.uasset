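; BP_Projectile is a pooled flipbook projectile that is activated by name at a start location and deals point damage on hit.
; Activation loads the named DataTable row asynchronously, caches its config for reuse, applies it and fires; only cached launches also trace at spawn.
; Blocks trigger impact and a damage sphere trace ignoring itself and the player.
; On deactivation, it messages the GameMode to return it to the pool.
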(event `self.ReceiveBeginPlay`
  (add `self.OnDeactivated` (`|CreateDelegate` :!event `OnDeactivated_Event`))
  (add `self.OnBlock` (`|CreateDelegate` :!event `OnBlock_Event`)))

(event `OnDeactivated_Event` :!signature `self.OnDeactivated`
  (params (Projectile :type "CPP_ProjectileParent Object Reference"))
  (message `/Game/_BottomlessPit/Blueprint/Interface/BPI_GameMode.I_GM_PoolProjectile` (`GameplayStatics.GetGameMode`) self))

(event `OnBlock_Event` :!signature `self.OnBlock`
  (params (Projectile :type "CPP_ProjectileParent Object Reference") (Hit :type "HitResult Structure (by ref)"))
  (`self.TriggerImpactAndDeactivate` Hit)
  (`self.DmgSphereTrace` (`.ImpactPoint` (`GameplayStatics.BreakHitResult` Hit))))

(event `/Game/_BottomlessPit/Blueprint/Interface/BPI_Actor.I_ActivateProjectile`
  (params (ProjectileName :type Name) (StartLoc :type "Vector Structure"))
  (bind _v_currentstartloc (`self.v_CurrentStartLoc`))
  (bind (_value _returnvalue) (`BlueprintMapLibrary.Map_Find` (`self.S_SaveProjectileStat`) (`self.n_CurrentProjectileName`)))
  (set `self.v_CurrentStartLoc` StartLoc)
  (set `self.n_CurrentProjectileName` ProjectileName)
  (if _returnvalue
    (`self.ApplyRuntimeConfig` _value)
    (`self.FireFromBP` _v_currentstartloc)
    (`self.DmgSphereTrace` _v_currentstartloc)
    (else
      (bind (_rowname _config) (`Util_BpAsyncProjectileFlipbooks.LoadProjectileFlipbooksRowAsync` (`self.DT_Projectile`) (`self.n_CurrentProjectileName`))
        (:`OnCompleted`
          (`BlueprintMapLibrary.Map_Add` (`self.S_SaveProjectileStat`) (`self.n_CurrentProjectileName`) _config)
          (`self.ApplyRuntimeConfig` _config)
          (`self.FireFromBP` (`self.v_CurrentStartLoc`)))))))

(event `DmgSphereTrace`
  (params (Start :type "Vector Structure"))
  (`self.SetActorEnableCollision` true)
  (bind _outhit (`KismetSystemLibrary.SphereTraceSingle` Start Start 40.0 "TraceTypeQuery3" false (`|MakeArray` self (`GameplayStatics.GetPlayerCharacter` 0) :!type "Actor Object Reference") "None" true (struct :`R` 1.0 :`A` 1.0) (struct :`G` 1.0 :`A` 1.0) 1.0))
  (bind (_bblockinghit _binitialoverlap _time _distance _location _impactpoint _normal _impactnormal _physmat _hitactor) (`GameplayStatics.BreakHitResult` _outhit))
  (`/Engine/EditorBlueprintResources/StandardMacros.IsValid` _hitactor
    (:`Is Valid`
      (`KismetSystemLibrary.PrintString` (`KismetSystemLibrary.GetDisplayName` _hitactor))
      (`self.TriggerImpactAndDeactivate` _outhit)
      (`GameplayStatics.ApplyPointDamage` _hitactor 1.0 (`self.K2_GetActorLocation` self) _outhit null self))))

(fn `UserConstructionScript`)