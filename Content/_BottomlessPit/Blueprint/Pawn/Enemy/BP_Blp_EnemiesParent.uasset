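; Parent Blueprint for pooled enemies in BottomlessPit, handling health, hit feedback and death.
; Health resets to max on BeginPlay and pool activation, and any damage triggers a flash and removes one health.
; On death it plays the resolved Death animation override, awards score and plays a hit sound, then signals completion when the animation finishes.
; Loaded animation sets are passed to the body's AnimInstance through an interface message.
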(event `self.ReceiveBeginPlay`
  (bind _healthcomp (`self.HealthComp`))
  (`self.BindEvent`)
  (`/Game/_BottomlessPit/Blueprint/Components/HitImpactComponent/AC_HitImpact.PawnInitHitImpactComponent` (`self.HitImpact Comp`))
  (`HealthComponent.SetCurrentHealth` _healthcomp (`HealthComponent.GetMaxHealth` _healthcomp)))

(event `self.OnPooledActivated`
  (bind _healthcomp (`self.HealthComp`))
  (`HealthComponent.SetCurrentHealth` _healthcomp (`HealthComponent.GetMaxHealth` _healthcomp)))

(event `self.OnPooledDeactivated`)

(event `self.ReceiveAnyDamage`
  (params (Damage :type "Float (single-precision)") (DamageType :type "DamageType Object Reference") (InstigatedBy :type "Controller Object Reference") (DamageCauser :type "Actor Object Reference"))
  (`/Game/_BottomlessPit/Blueprint/Components/HitImpactComponent/AC_HitImpact.StartDamagedFlash` (`self.HitImpact Comp`))
  (`HealthComponent.AddHealth` (`self.HealthComp`) -1.0))

(event `self.HealthComp.OnDead`
  (`self.BeginDeath`)
  (`PaperZDPlaySlotOverrideAction.PlayAnimationOverrideWithCallbacks` (`PaperZDAnimationComponent.AnimInstance` (`self.BodyAnim`)) (`.Death` (break `EnemyAnimResolved` (`self.ResolvedAnims`)))
    (:`then`
      (message `/Game/_BottomlessPit/Blueprint/Interface/BPI_GameMode.I_GM_Blp_AddScore` (`GameplayStatics.GetGameMode`) 250.0)
      (`/Game/_BottomlessPit/Blueprint/FunctionLibrary/BFL_GameFeels.StartSFX` "Hit"))
    (:`OnCompleted`
      (`self.Notify_DeathAnimFinished`))))

(event `OnAnimsReady_Event`
  (params (LoadedAnims :type "EnemyAnimResolved Structure (by ref)"))
  (message `/Game/_BottomlessPit/Blueprint/Interface/BPI_CharacterAnimation.I_E_SetAnim` (`PaperZDAnimationComponent.AnimInstance` (`self.BodyAnim`)) LoadedAnims))

(event `OnAnimsLoadFailed_Event`)

(fn `BindEvent`
  (add `self.OnAnimsReady` (`|CreateDelegate` :!event `OnAnimsReady_Event`))
  (add `self.OnAnimsLoadFailed` (`|CreateDelegate` :!event `OnAnimsLoadFailed_Event`)))

(fn `UserConstructionScript`)