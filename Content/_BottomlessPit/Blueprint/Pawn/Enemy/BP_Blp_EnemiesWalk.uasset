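; Pooled walking-enemy pawn that deals contact damage to the player when its capsule overlaps them.
; Restores full health on spawn and pool activation; any hit removes one health point and triggers a damage flash through HitImpactComp.
; Passes loaded animations to the body AnimInstance via an interface message.
; Death requests pool deactivation, plays a death override animation, then hides the actor and requests deactivation again on completion.
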(event `self.ReceiveBeginPlay`
  (bind _healthcomp (`self.HealthComp`))
  (`self.BindEvent`)
  (`/Game/_BottomlessPit/Blueprint/Components/HitImpactComponent/AC_HitImpact.PawnInitHitImpactComponent` (`self.HitImpact Comp`))
  (`HealthComponent.SetCurrentHealth` _healthcomp (`HealthComponent.GetMaxHealth` _healthcomp)))

(event `self.OnPooledActivated`
  (bind _healthcomp (`self.HealthComp`))
  (`self.SetActorHiddenInGame` false)
  (`HealthComponent.SetCurrentHealth` _healthcomp (`HealthComponent.GetMaxHealth` _healthcomp)))

(event `self.OnPooledDeactivated`)

(event `self.ReceiveAnyDamage`
  (params (Damage :type "Float (single-precision)") (DamageType :type "DamageType Object Reference") (InstigatedBy :type "Controller Object Reference") (DamageCauser :type "Actor Object Reference"))
  (`/Game/_BottomlessPit/Blueprint/Components/HitImpactComponent/AC_HitImpact.StartDamagedFlash` (`self.HitImpact Comp`))
  (`HealthComponent.AddHealth` (`self.HealthComp`) -1.0))

(event `self.HealthComp.OnDead`
  (`self.RequestDeactivate`)
  (`PaperZDPlaySlotOverrideAction.PlayAnimationOverrideWithCallbacks` (`PaperZDAnimationComponent.AnimInstance` (`self.BodyAnim`)) (`.Death` (break `EnemyAnimResolved` (`self.ResolvedAnims`)))
    (:`OnCompleted`
      (`self.SetActorHiddenInGame` true)
      (`self.RequestDeactivate`))))

(event `OnAnimsReady_Event`
  (params (LoadedAnims :type "EnemyAnimResolved Structure (by ref)"))
  (message `/Game/_BottomlessPit/Blueprint/Interface/BPI_CharacterAnimation.I_E_SetAnim` (`PaperZDAnimationComponent.AnimInstance` (`self.BodyAnim`)) LoadedAnims))

(event `OnAnimsLoadFailed_Event`)

(event `self.Capsule.OnComponentBeginOverlap`
  (params (OverlappedComponent :type "PrimitiveComponent Object Reference") (OtherActor :type "Actor Object Reference") (OtherComp :type "PrimitiveComponent Object Reference") (OtherBodyIndex :type Integer) (bFromSweep :type Boolean) (SweepResult :type "HitResult Structure (by ref)"))
  (if (== OtherActor (`GameplayStatics.GetPlayerCharacter` 0))
    (`GameplayStatics.ApplyDamage` OtherActor 1.0 null self)))

(fn `BindEvent`
  (add `self.OnAnimsReady` (`|CreateDelegate` :!event `OnAnimsReady_Event`))
  (add `self.OnAnimsLoadFailed` (`|CreateDelegate` :!event `OnAnimsLoadFailed_Event`)))

(fn `UserConstructionScript`)