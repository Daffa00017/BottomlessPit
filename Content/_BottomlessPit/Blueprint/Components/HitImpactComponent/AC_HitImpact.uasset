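; Actor component giving Paper2D characters and pawns hit reactions: sprite shake, damage color flash, stagger and knockback, initialized by the owner.
; Attack stats set shake strength, add to a stagger count and stack clamped knockback/knock-up.
; Reaching the stagger threshold enables stagger resistance and launches the character, using the registered damage causer for direction.
; Looping timers drive the shake, flash fade and stagger spin by directly modifying the flipbook sprite.
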(event `ChraInitHitImpactComponent`
  (params (OwnerChraObjectRef :type "Character Object Reference"))
  (bind (_damagedspriteflashcolor_r _damagedspriteflashcolor_g _damagedspriteflashcolor_b) (break `LinearColor` (`self.DamagedSpriteFlashColor`)))
  ;[1 1 1] Init Hit Impact Component (call this in beginplay of owner)
  (set `self.OwnerChraObjectRef` OwnerChraObjectRef)
  (set `self.CachedMovementComp` (`Actor.GetComponentByClass` OwnerChraObjectRef "/Script/Engine.PawnMovementComponent"))
  (set `self.CachedPrimitiveComp` (`Actor.GetComponentByClass` OwnerChraObjectRef "/Script/Engine.PrimitiveComponent"))
  (bind _output_get (set `self.Sprite` (`Actor.GetComponentByClass` OwnerChraObjectRef "/Script/Paper2D.PaperFlipbookComponent")))
  (set `self.v_SpriteBaseLoc` (`SceneComponent.RelativeLocation` _output_get))
  (bind _output_get_2 (set `self.BaseSpriteColor` (`PaperFlipbookComponent.SpriteColor` _output_get)))
  (bind (_r _g _b) (`KismetMathLibrary.BreakColor` _output_get_2))
  (set `self.f_BaseColor` (`KismetMathLibrary.MakeVector` _r _g _b))
  (set `self.f_DamagedColor` (`KismetMathLibrary.MakeVector` _damagedspriteflashcolor_r _damagedspriteflashcolor_g _damagedspriteflashcolor_b)))

(event `PawnInitHitImpactComponent`
  (bind _returnvalue (`self.GetOwner`))
  (bind (_damagedspriteflashcolor_r _damagedspriteflashcolor_g _damagedspriteflashcolor_b) (break `LinearColor` (`self.DamagedSpriteFlashColor`)))
  ;[1 1 1] Init Hit Impact Component (call this in beginplay of owner)
  (set `self.OwnerPawnObjectRef` _returnvalue)
  (set `self.CachedMovementComp` (`Actor.GetComponentByClass` _returnvalue "/Script/Engine.PawnMovementComponent"))
  (set `self.CachedPrimitiveComp` (`Actor.GetComponentByClass` _returnvalue "/Script/Engine.PrimitiveComponent"))
  (bind _output_get (set `self.Sprite` (`Actor.GetComponentByClass` _returnvalue "/Script/Paper2D.PaperFlipbookComponent")))
  (set `self.v_SpriteBaseLoc` (`SceneComponent.RelativeLocation` _output_get))
  (bind _output_get_2 (set `self.BaseSpriteColor` (`PaperFlipbookComponent.SpriteColor` _output_get)))
  (bind (_r _g _b) (`KismetMathLibrary.BreakColor` _output_get_2))
  (set `self.f_BaseColor` (`KismetMathLibrary.MakeVector` _r _g _b))
  (set `self.f_DamagedColor` (`KismetMathLibrary.MakeVector` _damagedspriteflashcolor_r _damagedspriteflashcolor_g _damagedspriteflashcolor_b)))

(event `ShakeSprite`
  ;[1 1 1] ShakeSprite Mechanic
  (set `self.f_ShakeIntensity` (`self.f_SpriteShakeIntensity`))
  (set `self.f_ShakeDuration` (`self.f_SpriteShakeDuration`))
  (set `self.f_ShakeCurrentDur` 0.0)
  (bind _returnvalue (`KismetSystemLibrary.K2_SetTimerDelegate` (delegate `Timer_ShakeSprite`) 0.01 true))
  (set `self.Th_ShakeSprite` _returnvalue))

(event `Timer_ShakeSprite`
  (bind (_v_spritebaseloc_x _v_spritebaseloc_y _v_spritebaseloc_z) (`KismetMathLibrary.BreakVector` (`self.v_SpriteBaseLoc`)))
  (bind _f_shakeintensity (`self.f_ShakeIntensity`))
  ;[1 1 1] ShakeSprite Mechanic
  (if (>= (`self.f_ShakeCurrentDur`) (`self.f_ShakeDuration`))
    (`KismetSystemLibrary.K2_ClearAndInvalidateTimerHandle` (`self.Th_ShakeSprite`))
    (set `self.f_ShakeCurrentDur` 0.0)
    (`SceneComponent.K2_SetRelativeLocation` (`self.Sprite`) (`self.v_SpriteBaseLoc`) false false)
    (else
      (set `self.f_ShakeCurrentDur` (+ (`self.f_ShakeCurrentDur`) 0.01))
      (`SceneComponent.K2_SetRelativeLocation` (`self.Sprite`) (`KismetMathLibrary.MakeVector` (`self.ResStagger_HalvenValue` (+ _v_spritebaseloc_x (`KismetMathLibrary.SelectFloat` _f_shakeintensity (* _f_shakeintensity -1.0) (`KismetMathLibrary.RandomBool`)))) _v_spritebaseloc_y _v_spritebaseloc_z) false false))))

(event `EndingDamageFlash`
  ;[1 1 1] Ending Damage Flash
  (set `self.f_TimerFlashDur` 0.0)
  (bind _returnvalue (`KismetSystemLibrary.K2_SetTimerDelegate` (`|CreateDelegate` :!event `EndDamagedFlash`) 0.05 true))
  (set `self.Th_DamageFlash` _returnvalue))

(event `ActivateHitImpact`
  (params (VFXName :type Name) (HitLoc :type "Vector Structure") (HittedActorLoc :type "Vector Structure"))
  ;[1 1 1] Activate Hit Impact
)

(event `StaggeredState`
  ;[1 1 1] Staggered (This part is when the owner get stagger, use for spawning fvx, rotating sprite, etc)
  (`self.RotateSprite`)
  (`KismetSystemLibrary.K2_SetTimerDelegate` (`|CreateDelegate` :!event `EndedStagger`) (`self.f_StaggerDuration`))
  (`self.ED_IsStaggered`))

(event `RotateSprite`
  ;[1 1 1] Rotate Sprite
  (set `self.f_RotateSpriteDur` 0.0)
  (bind _returnvalue (`KismetSystemLibrary.K2_SetTimerDelegate` (delegate `Timer_RotateSprite`) 0.02 true))
  (set `self.Th_RotateSprite` _returnvalue))

(event `Timer_RotateSprite`
  (bind _sprite (`self.Sprite`))
  (bind (_relativerotation_roll _relativerotation_pitch _relativerotation_yaw) (`KismetMathLibrary.BreakRotator` (`SceneComponent.RelativeRotation` _sprite)))
  ;[1 1 1] Rotate Sprite
  (set `self.f_RotateSpriteDur` (+ (`self.f_RotateSpriteDur`) 0.02))
  (if (>= (`self.f_RotateSpriteDur`) (`self.f_StaggerDuration`))
    (`KismetSystemLibrary.K2_ClearAndInvalidateTimerHandle` (`self.Th_RotateSprite`))
    (`SceneComponent.K2_SetRelativeRotation` :`self` (`self.Sprite`))
    (else
      (`SceneComponent.K2_SetRelativeRotation` _sprite (`KismetMathLibrary.MakeRotator` _relativerotation_roll _relativerotation_pitch (+ _relativerotation_yaw (* 360.0 0.02))) false false))))

(fn `ApplyStatAttack`
  (params (StructIn :type "/Game/_BottomlessPit/Blueprint/Components/HitImpactComponent/S_AttackStat Structure (by ref)"))
  (bind _structin (`local.StructIn`))
  (bind ((`ShouldShake?_26_729963C1415A7538BB7216B6A6F0F28F` _shouldshake_) (`ShakeIntensity_27_78BE26E541E71922DAEFD091ADD355B7` _shakeintensity) (`ShakeDuration_28_0D475CB94E00110CA7BB38AC37EC6C44` _shakeduration)) (break `/Game/_BottomlessPit/Blueprint/Components/HitImpactComponent/S_AttackStat` _structin))
  (bind ((`ShouldKnockback?_1_1C4C1CA943963442C261D5BC04D8C34B` _shouldknockback_) (`KnockUpMult_17_A84DF906438C94173C3D929B16B644FB` _knockupmult) (`KnockBackMult_18_CBBE34044D21DEA7DBEDC6974B76B652` _knockbackmult)) (break `/Game/_BottomlessPit/Blueprint/Components/HitImpactComponent/S_AttackStat` _structin))
  ;[1 1 1] Apply Sprite Shake Intensity from Stat
  (set `self.f_SpriteShakeIntensity` (`KismetMathLibrary.SelectFloat` _shakeintensity 0.0 _shouldshake_))
  (set `self.f_SpriteShakeDuration` (`KismetMathLibrary.SelectFloat` _shakeduration 0.0 _shouldshake_))
  ;[1 1 1] Do owner Use stagger mechanic?
  (if (`self.b_UseStaggerMechanic`)
    ;[1 1 1] Start Stagger function with stagger count from attack stat
    (`self.StartStaggered` (`.StaggerCount_32_12508E1C4E7022CFB80BBFB443D33E4C` (break `/Game/_BottomlessPit/Blueprint/Components/HitImpactComponent/S_AttackStat` _structin)))
    ;[1 1 1] Check if resist stagger
    (if (`self.b_CanResistStagger`)
      (`KismetSystemLibrary.PrintString` "Resist Stagger")
      (else
        ;[1 1 1] Apply Knockback multiplier (can stack but have max value)
        (set `self.f_KnockbackMult` (`KismetMathLibrary.FClamp` (`KismetMathLibrary.SelectFloat` (+ (`self.f_KnockbackMult`) _knockbackmult) 0.0 _shouldknockback_) 0.0 (`self.f_MaxKnockBackMult`)) :!label _label)
        (set `self.f_KnockUpMult` (`KismetMathLibrary.FClamp` (`KismetMathLibrary.SelectFloat` (+ (`self.f_KnockUpMult`) _knockupmult) 0.0 _shouldknockback_) 0.0 (`self.f_MaxKnockUpMult`)))))
    (else
      (goto _label))))

(fn `ChracterAttackKnockBack`
  (locals (KnockUpMultiplier :type "Float (double-precision)") (KnockBackMultiplier :type "Float (double-precision)"))
  (bind _damagedcauserref (`self.DamagedCauserRef`))
  (`Character.LaunchCharacter` (`self.OwnerChraObjectRef`) (+ (* (`KismetMathLibrary.Vector_Up`) (`self.f_KnockUpMult`)) (* (`self.CalculateHitDirection` (`Actor.K2_GetActorLocation` (select `bool` (`KismetSystemLibrary.IsValid` _damagedcauserref) :`false` (`self.OwnerChraObjectRef`) :`true` _damagedcauserref :!type "Actor Object Reference"))) (`self.f_KnockbackMult`))) true true)
  (set `self.f_KnockbackMult` 0.0)
  (set `self.f_KnockUpMult` 0.0))

(fn `ChraRegularKnockBack`
  (params (KnockUpMultiplier :type "Float (double-precision)") (KnockBackMultiplier :type "Float (double-precision)") (DamagedCauser :type "Actor Object Reference"))
  (locals (KnockUpMultiplier :type "Float (double-precision)") (KnockBackMultiplier :type "Float (double-precision)"))
  (bind _returnvalue (+ (* (`KismetMathLibrary.Vector_Up`) KnockUpMultiplier) (* (`self.CalculateHitDirection` (`Actor.K2_GetActorLocation` DamagedCauser)) KnockBackMultiplier)))
  (`Character.LaunchCharacter` (`self.OwnerChraObjectRef`) _returnvalue true true)
  (`KismetSystemLibrary.PrintString` (`KismetStringLibrary.Conv_VectorToString` _returnvalue) true true (struct :`R` 1.0 :`G` 0.013405 :`B` 0.212394 :`A` 1.0)))

(fn `EndDamagedFlash`
  (bind _output_get (set `self.f_TimerFlashDur` (+ (`self.f_TimerFlashDur`) 0.01)))
  (`PaperFlipbookComponent.SetSpriteColor` (`self.Sprite`) (make `LinearColor` (.x (`KismetMathLibrary.VLerp` (`self.f_BaseColor`) (`self.f_DamagedColor`) (`KismetMathLibrary.Lerp` (`self.f_FlashMultiplier`) 0.0 (/ _output_get (`self.f_DamageFlashDur`))))) (.y (`KismetMathLibrary.VLerp` (`self.f_BaseColor`) (`self.f_DamagedColor`) (`KismetMathLibrary.Lerp` (`self.f_FlashMultiplier`) 0.0 (/ _output_get (`self.f_DamageFlashDur`))))) (.z (`KismetMathLibrary.VLerp` (`self.f_BaseColor`) (`self.f_DamagedColor`) (`KismetMathLibrary.Lerp` (`self.f_FlashMultiplier`) 0.0 (/ _output_get (`self.f_DamageFlashDur`))))) 1.0))
  (if (>= (`self.f_TimerFlashDur`) (`self.f_DamageFlashDur`))
    (`PaperFlipbookComponent.SetSpriteColor` (`self.Sprite`) (`self.BaseSpriteColor`))
    (`KismetSystemLibrary.K2_ClearAndInvalidateTimerHandle` (`self.Th_DamageFlash`))
    (set `self.f_TimerFlashDur` 0.0)))

(fn `EndedStagger`
  (bind _output_get (set `self.b_IsStaggered` false)))

(fn `RegisterDamageCauser`
  (params (DamagedCauserIn :type "Actor Object Reference"))
  (`/Engine/EditorBlueprintResources/StandardMacros.IsValid` DamagedCauserIn
    (:`Is Valid`
      (`/Engine/EditorBlueprintResources/StandardMacros.IsValid` (`self.DamagedCauserRef`)
        (:`Is Valid`
          (if (not (== (`local.DamagedCauserIn`) (`self.DamagedCauserRef`)))
            (set `self.DamagedCauserRef` (`local.DamagedCauserIn`))))
        (:`Is Not Valid`
          (set `self.DamagedCauserRef` (`local.DamagedCauserIn`)))))))

(fn `StartDamagedFlash`
  (`PaperFlipbookComponent.SetSpriteColor` (`self.Sprite`) (`self.DamagedSpriteFlashColor`))
  (if (`KismetSystemLibrary.K2_IsTimerActiveHandle` (`self.Th_DamageFlash`))
    (`KismetSystemLibrary.K2_ClearAndInvalidateTimerHandle` (`self.Th_DamageFlash`)))
  (`self.EndingDamageFlash`))

(fn `StartStaggered`
  (params (AttackStaggerIn :type "Float (double-precision)"))
  (if (not (`self.b_CanResistStagger`))
    (bind _output_get (set `self.i_CurrentStaggerCount` (+ (`self.i_CurrentStaggerCount`) (`local.AttackStaggerIn`))))
    (if (>= (`self.i_CurrentStaggerCount`) (`self.i_CountToBeStaggered`))
      (set `self.b_CanResistStagger` true)
      (set `self.b_PendingStaggered` true)
      (`self.ChracterAttackKnockBack`)
      (bind _output_get_2 (set `self.b_IsStaggered` true)))))