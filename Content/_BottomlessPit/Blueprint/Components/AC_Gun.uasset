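; AC_Gun is a gun component that starts and stops firing and relays firing events to listeners through event dispatchers.
; StartShoot and StopShoot drive StartFire and StopFire, while shot-spawn and trigger-fired callbacks rebroadcast the shot direction and profile.
; Trigger permission and ammo checks query the owner through interface messages.
; TryConsumeAmmo only compares current ammo with the cost and deducts nothing.
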(event `StartShoot`
  (`self.StartFire`)
  (`self.ED_StartFire`))

(event `StopShoot`
  (`self.StopFire`))

(event `self.OnRequestSpawnShot`
  (params (ShotDir :type "Vector Structure") (ProjectileRowName :type Name) (bPenetrate :type Boolean) (ProjectileScale :type "Float (single-precision)") (DamagePerProjectile :type "Float (single-precision)") (ProjectileLifeSecondsOverride :type "Float (single-precision)"))
  (`self.ED_OnFiringProjectile` ShotDir))

(event `self.OnTriggerFired`
  (params (Profile :type "FireModeProfile Structure (by ref)"))
  (`self.ED_OnTriggeredFired` Profile))

(fn `CanBeginTrigger`
  (returns (ReturnValue :type Boolean))
  (bind _true_ (message `/Game/_BottomlessPit/Blueprint/Interface/BPI_Player.I_P1_CanFire` (`self.GetOwner`)))
  (return _true_))

(fn `TryConsumeAmmo`
  (params (Cost :type Integer))
  (returns (ReturnValue :type Boolean))
  (bind _currentammo (message `/Game/_BottomlessPit/Blueprint/Interface/BPI_Player.I_P1_GetPlayerCurrAmmo` (`self.GetOwner`)))
  (if (>= _currentammo Cost)
    (return true)
    (else
      (return false))))