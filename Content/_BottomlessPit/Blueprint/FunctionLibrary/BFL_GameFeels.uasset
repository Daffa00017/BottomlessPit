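; Blueprint function library of global game-feel shortcuts for camera shake, hitstop, sound effects, music, VFX and combo tracking.
; Camera shake plays a fixed medium fire shake class on player 0's camera manager at a given scale.
; Every other function forwards its arguments to the Game Mode through interface messages, so callers need no direct reference to the systems that carry out the effects.
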(fn `AddCombo`
  (params (ComboInput :type "Float (double-precision)"))
  (message `/Game/_BottomlessPit/Blueprint/Interface/BPI_GameMode.I_GM_Blp_AddCombo` (`GameplayStatics.GetGameMode` null) ComboInput))

(fn `StartBgm`
  (message `/Game/_BottomlessPit/Blueprint/Interface/BPI_GameMode.I_GM_StartBgm` (`GameplayStatics.GetGameMode` null)))

(fn `StartBgmMainMenu`
  (message `/Game/_BottomlessPit/Blueprint/Interface/BPI_GameMode.I_GM_StartBgmMainMenu` (`GameplayStatics.GetGameMode` null)))

(fn `StartCamShake`
  (params (Scale :type "Float (single-precision)" :default 1.0))
  (`LegacyCameraShake.StartLegacyCameraShake` (`PlayerController.PlayerCameraManager` (`GameplayStatics.GetPlayerController` null)) "/Game/_BottomlessPit/Asset/BottomlessPit/CamShake/CS_Fire_Medium.CS_Fire_Medium_C" Scale))

(fn `StartHitstop`
  (params (Dur :type "Float (double-precision)") (MinDil :type "Float (double-precision)"))
  (message `/Game/_BottomlessPit/Blueprint/Interface/BPI_GameMode.I_GM_StartHitstopSimple` (`GameplayStatics.GetGameMode` null) Dur MinDil))

(fn `StartHitstopAdvance`
  (params (Dur :type "Float (double-precision)" :default 0.1) (MinDil :type "Float (double-precision)" :default 0.1) (Curve :type "CurveFloat Object Reference") (Intensity :type "Float (double-precision)" :default 1.0))
  (message `/Game/_BottomlessPit/Blueprint/Interface/BPI_GameMode.I_GM_StartHitstopAdvance` (`GameplayStatics.GetGameMode` null) Dur MinDil Curve Intensity))

(fn `StartSFX`
  (params (SFXName :type Name))
  (message `/Game/_BottomlessPit/Blueprint/Interface/BPI_GameMode.I_GM_ActivateSFX` (`GameplayStatics.GetGameMode` null) SFXName))

(fn `StartVFX`
  (params (ImpactLoc :type "Vector Structure") (AnimName :type Name))
  (message `/Game/_BottomlessPit/Blueprint/Interface/BPI_GameMode.I_GM_StartFVX` (`GameplayStatics.GetGameMode` null) ImpactLoc AnimName))

(fn `StartVFXTransform`
  (params (Transform :type "Transform Structure") (AnimName :type Name))
  (message `/Game/_BottomlessPit/Blueprint/Interface/BPI_GameMode.I_GM_ActivFVXTransform` (`GameplayStatics.GetGameMode` null) Transform AnimName))

(fn `StopBgm`
  (message `/Game/_BottomlessPit/Blueprint/Interface/BPI_GameMode.I_GM_StopBgm` (`GameplayStatics.GetGameMode` null)))

(fn `StopBgmMainMenu`
  (message `/Game/_BottomlessPit/Blueprint/Interface/BPI_GameMode.I_GM_StopBgmMainMenu` (`GameplayStatics.GetGameMode` null)))

(fn `StopCombo`
  (message `/Game/_BottomlessPit/Blueprint/Interface/BPI_GameMode.I_GM_Blp_StopCombo` (`GameplayStatics.GetGameMode` null)))