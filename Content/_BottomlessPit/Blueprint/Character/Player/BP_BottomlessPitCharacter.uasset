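; Player character for BottomlessPit, a sprite-based falling game where the jump input fires ammo-limited projectiles from below the player.
; FireComponent applies data-driven fire modes, gates shots through jumping and requests projectiles from the GameMode.
; A stomp sensor damages enemies, while down-smash ramps gravity and sensor size by timeline and breaks platforms on impact.
; Health drives mercy invincibility, death and restart, relayed by interfaces to HUD, controller and level generator.
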(event OnHealthChange(Health)
  (params (NewHealth :type Float%20%28single-precision%29))
  ;[0.8941 0.2251 0.6132 0.5] Health Event
  (Class|BPIHUDandUI|IUIonHealthChange(Message) (Variables|Default|GetRef_HUD) NewHealth))

(event OnMaxHealthChange(Health)
  (params (NewMaxHealth :type Float%20%28single-precision%29))
  ;[0.8941 0.2251 0.6132 0.5] Health Event
  (Class|BPIHUDandUI|IUIonMaxHealthChange(Message) (Variables|Default|GetRef_HUD) NewMaxHealth))

(event OnDead(Health)
  (bind _charactermovement (Variables|Character|GetCharacterMovement))
  ;[0.8941 0.2251 0.6132 0.5] Health Event
  (if (not (Variables|Default|GetIsDead))
    (Variables|Default|SetIsDead true)
    (Class|BPIPlayerController|IPconDead(Message) (Game|GetPlayerController 0) true)
    (Class|BPIActor|IBlpDeactivatePlatform(Message) (Variables|Default|GetRef_LevelGenerator) false)
    (Pawn|Components|CharacterMovement|SetMovementMode _charactermovement "MOVE_None" 0)
    (Components|Movement|StopMovementImmediately _charactermovement)
    (CallFunction|StopBgm)
    (CallFunction|StartSFX "PlayerDeath")
    (CallFunction|StartBgmMainMenu)))

(event OnComponentBeginOverlap(StompSensor)
  (params (OverlappedComponent :type Primitive%20Component%20Object%20Reference) (OtherActor :type Actor%20Object%20Reference) (OtherComp :type Primitive%20Component%20Object%20Reference) (OtherBodyIndex :type Integer) (bFromSweep :type Boolean) (SweepResult :type Hit%20Result%20Structure%20%28by%20ref%29))
  (if (Actor|ActorHasTag OtherActor "Enemies")
    (if (not (and (Actor|ActorHasTag OtherActor "Immune") (not (Variables|Default|GetIsSmashingDown))))
      (Game|Damage|ApplyDamage OtherActor 1.0 0 0)
      (Default|ChraRegularKnockBack (Variables|Default|GetAC_HitImpact) 8e+02 1.5e+02 OtherActor)
      (CallFunction|StartCamShake 2.5)
      (if (Variables|Default|GetIsSmashingDown)
        (Audio|Components|Audio|Stop (Variables|Default|GetTL_SmashingDownGravity))
        (CallFunction|SmashingDown)
        (CallFunction|StartHitstop 0.075 0.15)))))

(event OnComponentBeginOverlap(CapsuleComponent)
  (params (OverlappedComponent :type Primitive%20Component%20Object%20Reference) (OtherActor :type Actor%20Object%20Reference) (OtherComp :type Primitive%20Component%20Object%20Reference) (OtherBodyIndex :type Integer) (bFromSweep :type Boolean) (SweepResult :type Hit%20Result%20Structure%20%28by%20ref%29))
  (if (and (Actor|ActorHasTag OtherActor "Enemies") (CallFunction|IsEnemyBelowPlayer OtherActor))
    (Game|Damage|ApplyDamage self 1.0 0 OtherActor :!label _label)
    (elif (Actor|ActorHasTag OtherActor "Immune")
      (goto _label))))

(event EDonTriggeredFired(FireComponent)
  (params (ProfileIn :type Fire%20Mode%20Profile%20Structure))
  ;[0.15 0.15 0.15 0.5] FireEvent
  (CallFunction|SetCurrentAmmo (Utilities|Struct|BreakFireModeProfile ProfileIn))
  (CallFunction|StartVFXTransform (Math|Transform|MakeTransform (- (CallFunction|GetCapsuleBottomLoc) "0.000000,0.000000,20.000000") "0, 0, 0" "1.000000,1.000000,1.000000") "BlpPrpjectileSpawn")
  (CallFunction|StartCamShake 0.6)
  (CallFunction|StartSFX "Shoot"))

(event EDonFiringProjectile(FireComponent)
  (params (ShootDir :type Vector :default "0, 0, 0"))
  ;[0.15 0.15 0.15 0.5] FireEvent
  (|CG_PlayJumpAnim
    (:execute
      (Class|BPIGameMode|IGMActivateProjectile(Message) (Game|GetGameMode) (Utilities|Struct|BreakFireModeProfile (Class|CPPGunComponent|GetCurrentProfile (Variables|Default|GetFire%20Component))) (- (CallFunction|GetCapsuleBottomLoc) "0.000000,0.000000,20.000000")))))

(event Custom|OnMovementStateChanged_Event
  (params (OldState :type EE_PlayerMovementState%20Enum :default "Idle") (NewState :type EE_PlayerMovementState%20Enum :default "Idle"))
  ;[0.15 0.15 0.15 0.5] Movement
  (Class|BPICharacterAnimation|ISetMovementState(Message) (Variables|/Script/PaperZD.PaperZDAnimationComponent|GetAnimInstance (Variables|Default|GetAnimationComponent)) NewState))

(event Custom|OnMoveAxisUpdatedDelegate_Event
  (params (Axis :type Float%20%28single-precision%29) (SpeedX :type Float%20%28single-precision%29))
  ;[0.15 0.15 0.15 0.5] Input
)

(event Custom|StartMercySpriteInvicible
  ;[0.8941 0.2251 0.6132 0.5] Health Event
  (|MercyInvicibleEvent))

(event Custom|AsyncPlayerAnim
  (params (RowName :type Name))
  (bind _anim (|LoadPlayerAnimRowAsync (Variables|Default|GetDT_PlayerAnim) RowName 0)
    (:OnCompleted
      (bind _output_get (Variables|Default|Sets_PlayerAnim _anim))
      (Class|BPICharacterAnimation|ISetPlayerAnim(Message) (Variables|Default|GetAnimReff) _output_get))))

(event Custom|TestingWeapon
  (bind _dt_firemode (Variables|Default|GetDT_FireMode))
  (bind _outrownames (DataTable|GetDataTableRowNames _dt_firemode))
  (bind _resolved (|LoadFireModeRowAsync _dt_firemode (.OutItem (Utilities|Array|Random _outrownames)))
    (:OnCompleted
      (CallFunction|ApplyFireMode (Utilities|Struct|BreakFireModeResolved _resolved)))))

(event Custom|OnDashStartedEvent_Event
  (params (Value :type Float%20%28single-precision%29))
  ;[0.15 0.15 0.15 0.5] Input
)

(event Custom|OnDashCompletedEvent_Event
  ;[0.15 0.15 0.15 0.5] Input
)

(event Custom|OnJumpStartedEvent_Event
  (params (Value :type Float%20%28single-precision%29))
  ;[0.15 0.15 0.15 0.5] Input
  (if (not (Variables|Default|GetIsDead))
    (Class|CPPDownwellLiteCharacter|StartStompWatch)
    (Default|StartShoot (Variables|Default|GetFire%20Component))))

(event Custom|OnJumpCompletedEvent_Event
  ;[0.15 0.15 0.15 0.5] Input
  (Default|StopShoot (Variables|Default|GetFire%20Component)))

(event Custom|OnDownSmashStartedEvent_Event
  (params (Value :type Float%20%28single-precision%29))
  ;[0.15 0.15 0.15 0.5] Input
  (if (Variables|Default|GetIsUpdatingGravity)
    (Variables|/Script/Engine.CharacterMovementComponent|SetGravityScale (Variables|Character|GetCharacterMovement) (* (Variables|Default|GetOriGravityScale) 1e+01))
    (Components|Box|SetBoxExtent (Variables|Default|GetStompSensor) (* (Variables|Default|Getv_StompOriExtent) 2.0) false)
    (else
      (|UpdateGravitySmashDown))))

(event Custom|OnDownSmashCompletedEvent_Event
  ;[0.15 0.15 0.15 0.5] Input
)

(event Custom|ClearCDCanJump
  ;[0.15 0.15 0.15 0.5] Movement
  (Variables|Default|Setb_CanJump true))

(event Custom|FallingDownAnim
  (bind _v_spriteoriginalloc (Variables|Default|Getv_SpriteOriginalLoc))
  (bind _curvalue (|DOVector3D "" 1.5 (+ _v_spriteoriginalloc "0.000000,0.000000,1500.000000") _v_spriteoriginalloc "Linear" false)
    (:OnUpdate
      (Transformation|SetRelativeLocation (Variables|Default|GetSprite) _curvalue false false))))

(event EventBeginPlay
  ;[0.15 0.15 0.15 0.5] Actor Event
  (CallFunction|BindEvent)
  (CallFunction|SetupBeginplay)
  (CallFunction|FallingDownAnim)
  (Default|ChraInitHitImpactComponent (Variables|Default|GetAC_HitImpact) self)
  (CallFunction|StartBgmMainMenu))

(event Collision|EventActorBeginOverlap
  (params (OtherActor :type Actor%20Object%20Reference))
  ;[0.15 0.15 0.15 0.5] Actor Event
)

(event EventIP1PlayeronRestart
  ;[0.15 0.15 0.15 0.5] Interface
  (|CG_OnPlayerRestart))

(event EventIP1PlayeronFirstInput
  ;[0.15 0.15 0.15 0.5] Interface
  (|CG_OnPlayerFirstInput))

(event EventIP1BlpRegisterCamera
  (params (Ref :type Actor%20Object%20Reference))
  (bind _output_get (Variables|Default|SetRef_Camera Ref))
  (Class|BPIActor|IBlpRegisterCamera(Message) (Variables|Default|GetRef_LevelGenerator) _output_get))

(event EventIP1SetCurrentAmmo
  (params (AmmoCostPerShot :type Integer))
  (CallFunction|SetCurrentAmmo AmmoCostPerShot))

(event EventIP1SetFireMode
  (params (StructIn :type Fire%20Mode%20Resolved%20Structure))
  (CallFunction|ApplyFireMode (Utilities|Struct|BreakFireModeResolved StructIn)))

(event EventIP1IsDoneJump
  (params (True? :type Boolean))
  (Class|BPICharacterAnimation|ISetIsDoneJump(Message) (Variables|Default|GetAnimReff) True?))

(event EventIP1BlpRegisterLaneLevel
  (params (Ref :type Actor%20Object%20Reference))
  ;[0.15 0.15 0.15 0.5] Interface
  (Variables|Default|SetRef_LevelGenerator Ref))

(event EventCustomEventonLanded
  (params (HitResult :type Hit%20Result%20Structure))
  ;[0.15 0.15 0.15 0.5] Movement
  (|PlayAnimationOverridewithCallbacks (Variables|Default|GetAnimReff) (Utilities|Struct|BreakPlayerAnimResolved (Variables|Default|Gets_PlayerAnim)) "DefaultSlot" 1.0 0.0
    (:then
      (Class|BPIGameMode|IGMBlpStopScore(Message) (Game|GetGameMode))
      (Class|BPICharacterAnimation|ISetFallingOfLedge(Message) (Variables|Default|GetAnimReff) false)
      (Audio|Components|Audio|Stop (Variables|Default|GetTL_SmashingDownGravity))
      (CallFunction|SmashingDown)
      (Class|BPICharacterAnimation|ISetIsDoneJump(Message) (Variables|Default|GetAnimReff) false))
    (:OnCompleted
      (Class|BPICharacterAnimation|ISetIsDoneJump(Message) (Variables|Default|GetAnimReff) false))))

(event EventOnWalkingOffLedge
  (params (PreviousFloorImpactNormal :type Vector%20%28by%20ref%29 :default "0, 0, 0") (PreviousFloorContactNormal :type Vector%20%28by%20ref%29 :default "0, 0, 0") (PreviousLocation :type Vector%20%28by%20ref%29 :default "0, 0, 0") (TimeDelta :type Float%20%28single-precision%29))
  ;[0.15 0.15 0.15 0.5] Movement
  (Class|BPICharacterAnimation|ISetFallingOfLedge(Message) (Variables|Default|GetAnimReff) true)
  (Class|CPPDownwellLiteCharacter|StartStompWatch)
  (Class|BPICharacterAnimation|ISetMovementState(Message) (Variables|Default|GetAnimReff) "Jump"))

(event Game|Damage|EventAnyDamage
  (params (Damage :type Float%20%28single-precision%29) (DamageType :type Damage%20Type%20Object%20Reference) (InstigatedBy :type Controller%20Object%20Reference) (DamageCauser :type Actor%20Object%20Reference))
  ;[0.8941 0.2251 0.6132 0.5] Health Event
  (|CheckIfHasMercy)
  (Class|HealthComponent|AddHealth (Variables|Default|GetHealth) (* Damage -1.0))
  (Utilities|IsValid DamageCauser
    (:Is%20Valid
      (Default|ChraRegularKnockBack (Variables|Default|GetAC_HitImpact) 8e+02 4e+02 DamageCauser)
      (CallFunction|StartHitstop 0.5 0.15)
      (CallFunction|StartCamShake 4.0))))

(event EventIP1PlayGameOverSequence
  ;[0.8941 0.2251 0.6132 0.5] Health Event
  (CallFunction|StartVFXTransform (Math|Transform|MakeTransform (- (Transformation|GetActorLocation (Game|GetPlayerCharacter 0)) "0.000000,0.000000,5.000000") "0, 0, 0" "1.000000,1.000000,1.000000") "BlpGameOver")
  (Utilities|AbpJumptoNode "JumpDeath")
  (Utilities|FlowControl|Delay 1.0)
  (Class|BPIHUDandUI|IUIonDeath(Message) (Variables|Default|GetRef_HUD)))

(event EventIP1ReadytoRestart
  (params (True? :type Boolean))
  ;[0.15 0.15 0.15 0.5] Interface
  (Variables|Default|SetIsReadyToRestart True?))

(event EventIP1ApplyAttackStat
  (params (AttackStat :type S%20Attack%20Stat%20Structure))
  ;[0.15 0.15 0.15 0.5] Interface
  (Default|ApplyStatAttack (Variables|Default|GetAC_HitImpact) AttackStat))

(event Input|KeyboardEvents|DebugKeyZ
  (params (Key :type Key%20Structure :default "None") (ActionValue :type Input%20Action%20Value%20Structure))
  ;[0.15 0.15 0.15 0.5] Input
  (:Pressed
    (Game|Damage|ApplyDamage self 4.0 0 0)))

(event Input|KeyboardEvents|DebugKeyF
  (params (Key :type Key%20Structure :default "None") (ActionValue :type Input%20Action%20Value%20Structure))
  ;[0.15 0.15 0.15 0.5] Input
  (:Pressed
    (|TrySpawnFireModePercentage)))

(fn ConstructionScript)

(fn BindEvent
  (EventDispatchers|BindEventtoOnMoveAxisUpdatedDelegate (EventDispatchers|CreateEvent :!event Custom|OnMoveAxisUpdatedDelegate_Event))
  (EventDispatchers|BindEventtoOnMovementStateChanged (EventDispatchers|CreateEvent :!event Custom|OnMovementStateChanged_Event))
  (EventDispatchers|BindEventtoOnDashStartedEvent (EventDispatchers|CreateEvent :!event Custom|OnDashStartedEvent_Event))
  (EventDispatchers|BindEventtoOnDashCompletedEvent (EventDispatchers|CreateEvent :!event Custom|OnDashCompletedEvent_Event))
  (EventDispatchers|BindEventtoOnJumpStartedEvent (EventDispatchers|CreateEvent :!event Custom|OnJumpStartedEvent_Event))
  (EventDispatchers|BindEventtoOnJumpCompletedEvent (EventDispatchers|CreateEvent :!event Custom|OnJumpCompletedEvent_Event))
  (EventDispatchers|BindEventtoOnDownSmashStartedEvent (EventDispatchers|CreateEvent :!event Custom|OnDownSmashStartedEvent_Event))
  (EventDispatchers|BindEventtoOnDownSmashCompletedEvent (EventDispatchers|CreateEvent :!event Custom|OnDownSmashCompletedEvent_Event)))

(fn SetupBeginplay
  (bind _returnvalue (Game|GetGameMode))
  (bind _health (Variables|Default|GetHealth))
  (bind _returnvalue_2 (Class|HealthComponent|GetMaxHealth _health))
  (Variables|Default|SetIsDead false)
  (Variables|Default|Setv_SpriteOriginalLoc (Variables|/Script/Engine.SceneComponent|GetRelativeLocation (Variables|Default|GetSprite)))
  (Variables|Default|Setv_PLayerOriginLoc (Transformation|GetActorLocation))
  (Variables|Default|SetRef_HUD (HUD|GetHUD (Game|GetPlayerController 0)))
  (Class|HealthComponent|SetCurrentHealth _health _returnvalue_2)
  (Class|BPIHUDandUI|IUIonMaxHealthChange(Message) (Variables|Default|GetRef_HUD) _returnvalue_2)
  (Variables|Default|SetLcs_SpriteOGColor (Class|PaperFlipbookComponent|GetSpriteColor (Variables|Default|GetSprite)))
  (bind _output_get (Variables|Default|SetAnimReff (Variables|/Script/PaperZD.PaperZDAnimationComponent|GetAnimInstance (Variables|Default|GetAnimationComponent))))
  (Class|BPICharacterAnimation|ISetFallingOfLedge(Message) _output_get true)
  (Class|PaperZDAnimInstance|JumptoNode (Variables|Default|GetAnimReff) "Jump_Idle" "Locomotion")
  (CallFunction|AsyncPlayerAnim "BlpMC")
  (Class|BPICharacterAnimation|IUseMoveAxis(Message) (Variables|Default|GetAnimReff) false)
  (Pawn|Components|CharacterMovement|SetMovementMode (Variables|Character|GetCharacterMovement) "MOVE_Falling" 0)
  (Class|BPICharacterAnimation|ISetMovementState(Message) (Variables|Default|GetAnimReff) "Jump")
  (Class|CPPDownwellLiteCharacter|StartStompWatch)
  (Variables|Default|Setv_StompOriExtent (Variables|/Script/Engine.BoxComponent|GetBoxExtent (Variables|Default|GetStompSensor)))
  (Class|BPIGameMode|IGMSpawnFVX(Message) _returnvalue 4)
  (Class|BPIGameMode|IGMSpawnProjectile(Message) _returnvalue 15)
  (Class|BPIGameMode|IGMSpawnFireMode(Message) _returnvalue 3))

(fn SmashingDown
  (if (Variables|Default|GetIsSmashingDown)
    (Variables|Default|Setb_CanJump false)
    (Variables|Default|SetIsSmashingDown false)
    (|CG_Platformdamage
      (:execute2
        (Variables|/Script/Engine.CharacterMovementComponent|SetGravityScale (Variables|Character|GetCharacterMovement) (Variables|Default|GetOriGravityScale))
        (CallFunction|StartVFXTransform (Math|Transform|MakeTransform (CallFunction|GetCapsuleBottomLoc) "0, 0, 0" "1.000000,1.000000,1.000000") "SlamSmoke")
        (Utilities|Time|SetTimerbyEvent (EventDispatchers|CreateEvent :!event Custom|ClearCDCanJump) (Variables|Default|Getf_JumpCdAfterSmash))
        (CallFunction|StartCamShake 2.5)
        (Components|Box|SetBoxExtent (Variables|Default|GetStompSensor) (Variables|Default|Getv_StompOriExtent) false)))
    (else
      (CallFunction|StartVFXTransform (Math|Transform|MakeTransform (CallFunction|GetCapsuleBottomLoc) "0, 0, 0" "1.000000,1.000000,1.000000") "LandSmoke"))))

(fn GetCapsuleBottomLoc
  (bind _returnvalue (Transformation|GetActorLocation))
  (return (Math|Vector|MakeVector (.x _returnvalue) (.y _returnvalue) (- (.z _returnvalue) (Components|Capsule|GetScaledCapsuleHalfHeight (Variables|Default|GetCapsuleComponent))))))

(fn RestartBeginplay
  (bind _returnvalue (Transformation|GetActorLocation))
  (bind _maxammocount (Variables|Default|GetMaxAmmoCount))
  (bind _health (Variables|Default|GetHealth))
  (bind _returnvalue_2 (Class|HealthComponent|GetMaxHealth _health))
  (Pawn|Components|CharacterMovement|SetMovementMode (Variables|Character|GetCharacterMovement) "MOVE_Falling" 0)
  (Variables|Default|SetIsDead false)
  (Transformation|SetActorLocation (Math|Vector|MakeVector (.x (Variables|Default|Getv_PLayerOriginLoc)) (.y _returnvalue) (.z _returnvalue)) false false)
  (Class|HealthComponent|SetCurrentHealth _health _returnvalue_2)
  (Class|BPIHUDandUI|IUIonMaxHealthChange(Message) (Variables|Default|GetRef_HUD) _returnvalue_2)
  (Class|BPICharacterAnimation|ISetFallingOfLedge(Message) (Variables|Default|GetAnimReff) true)
  (Class|BPICharacterAnimation|IUseMoveAxis(Message) (Variables|Default|GetAnimReff) false)
  (Variables|Default|SetJumpMaxCount (+ (Variables|Default|GetMaxAmmoCount) 1))
  (Variables|Default|SetCurrentAmmoCount _maxammocount)
  (Class|BPIHUDandUI|IUIBlponMaxAmmoChange(Message) (Variables|Default|GetRef_HUD) _maxammocount))

(fn IsEnemyBelowPlayer
  (params (ActorRefIn :type Actor%20Object%20Reference))
  (bind _capsulecomponent (Variables|Default|GetCapsuleComponent))
  (return (< (- (.z (Transformation|GetWorldLocation _capsulecomponent)) (Components|Capsule|GetScaledCapsuleHalfHeight _capsulecomponent)) (.z (Transformation|GetActorLocation ActorRefIn)))))

(fn SetCurrentAmmo
  (params (AmmoCost :type Integer))
  (bind _output_get (Variables|Default|SetCurrentAmmoCount (- (Variables|Default|GetCurrentAmmoCount) AmmoCost)))
  (Class|BPIHUDandUI|IUIBlponCurrentAmmoChange(Message) (Variables|Default|GetRef_HUD) _output_get))

(fn SetMaxAmmo
  (bind _output_get (Variables|Default|SetMaxAmmoCount (Utilities|Struct|BreakFireModeProfile (Class|CPPGunComponent|GetCurrentProfile (Variables|Default|GetFire%20Component)))))
  (Variables|Default|SetJumpMaxCount (+ _output_get 99))
  (Class|BPIHUDandUI|IUIBlponMaxAmmoChange(Message) (Variables|Default|GetRef_HUD) (Variables|Default|GetMaxAmmoCount))
  (Variables|Default|SetCurrentAmmoCount (Variables|Default|GetMaxAmmoCount)))

(fn ApplyFireMode
  (params (Profile :type Fire%20Mode%20Profile%20Structure%20%28by%20ref%29))
  (Class|CPPGunComponent|ApplyFireMode (Variables|Default|GetFire%20Component) Profile)
  (CallFunction|SetMaxAmmo)
  (Development|PrintString (Utilities|String|ToString(Name) (Utilities|Struct|BreakFireModeProfile Profile))))

(fn IP1CanFire
  (Utilities|OnFireBranch
    (:Exec
      (return true))))

(fn IP1GetCurrentAmmoPercent
  (return (Math|Float|Clamp(Float) (/ (Variables|Default|GetCurrentAmmoCount) (Variables|Default|GetMaxAmmoCount)))))

(fn IP1GetPlayerCurrAmmo
  (return (Variables|Default|GetCurrentAmmoCount)))

(fn IP1GetPlayerRef
  (return self))

(fn IP1IsPlayerDead
  (return (Variables|Default|GetIsDead)))

(fn IP1IsReadytoRestart
  (return (Variables|Default|GetIsReadyToRestart)))