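; BP_FireMode is a pooled pickup that gives the player a random fire mode from a data table.
; On activation it async-loads and caches the row, sets its Paper2D sprite, and launches upward on a timeline, starting a short timer.
; Player overlap, when allowed, sends the fire mode by interface, triggers VFX and fades it out.
; Otherwise a lifetime timeline drives sprite alpha, then returns it to the GameMode's pool.
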(event `self.ReceiveBeginPlay`
  (`self.SetActorTickEnabled` false)
  (`self.SetActorHiddenInGame` false)
  (`self.K2_SetActorLocation` (0.0 0.0 0.0))
  (`self.SetActorEnableCollision` false))

(event `OnActorActivatedByPool`
  (bind _dt_firemode (`self.DT_FireMode`))
  (bind _outrownames (`DataTableFunctionLibrary.GetDataTableRowNames` _dt_firemode))
  (bind _output_get (set `self.Fn_CurrentWeaponName` (`KismetArrayLibrary.Array_Random` _outrownames)))
  (bind (_value _returnvalue) (`BlueprintMapLibrary.Map_Find` (`self.Map_CachedProfile`) _output_get))
  (if _returnvalue
    (set `self.S_CurrentFireMode` _value)
    (`PaperSpriteComponent.SetSprite` (`self.PaperSprite`) (`.PickupSprite` (break `FireModeResolved` _value)))
    (else
      (bind (_rowname _resolved) (`Util_BpAsyncFireModeProfile.LoadFireModeRowAsync` _dt_firemode _output_get)
        (:`OnCompleted`
          (set `self.S_CurrentFireMode` _resolved)
          (`PaperSpriteComponent.SetSprite` (`self.PaperSprite`) (`.PickupSprite` (break `FireModeResolved` _resolved)))
          (`BlueprintMapLibrary.Map_Add` (`self.Map_CachedProfile`) _output_get _resolved))))))

(event `self.Box.OnComponentBeginOverlap`
  (params (OverlappedComponent :type "PrimitiveComponent Object Reference") (OtherActor :type "Actor Object Reference") (OtherComp :type "PrimitiveComponent Object Reference") (OtherBodyIndex :type Integer) (bFromSweep :type Boolean) (SweepResult :type "HitResult Structure (by ref)"))
  (if (and (`self.b_CanBeOverlapped`) (== OtherActor (`GameplayStatics.GetPlayerCharacter` 0)))
    (set `self.b_CanBeOverlapped` false)
    (message `/Game/_BottomlessPit/Blueprint/Interface/BPI_Player.I_P1_SetFireMode` (`GameplayStatics.GetPlayerCharacter` 0) (`self.S_CurrentFireMode`))
    (`self.OnOverlapEvent`)
    (`self.ActorDisappear` 3.0)))

(event `/Game/_BottomlessPit/Blueprint/Interface/BPI_Actor.I_ActivateFireMode`
  (params (StartLoc :type "Vector Structure"))
  (set `self.v_CurrectLoc` StartLoc)
  (`self.StartLaunch` 1.5)
  (`self.OnActorActivatedByPool`)
  (`KismetSystemLibrary.K2_SetTimerDelegate` (`|CreateDelegate` :!event `ActivateCanOverlapped`) 0.45))

(event `ActorDisappear`
  (params (PlayRate :type "Float (double-precision)" :default 1.0))
  (`TimelineComponent.SetPlayRate` (`self.TL_Disappear`) (* 1.0 PlayRate))
  (`TimelineComponent.Stop` (`self.TL_LifeTime`))
  (bind (_direction _alpha) (`Timeline|TL_Disappear` :!via `PlayFromStart`)
    (:`Update`
      (`PaperSpriteComponent.SetSpriteColor` (`self.PaperSprite`) (`KismetMathLibrary.MakeColor` 1.0 1.0 1.0 _alpha)))
    (:`Finished`
      (`self.K2_SetActorLocation` (0.0 0.0 0.0) :!label _label)
      (`self.SetActorHiddenInGame` true)
      (message `/Game/_BottomlessPit/Blueprint/Interface/BPI_GameMode.I_GM_PoolFireMode` (`GameplayStatics.GetGameMode`) self)
      (set `self.b_CanBeOverlapped` false)
      (`self.SetActorEnableCollision` false))))

(event `ForceToPool`
  (goto _label))

(event `StartLaunch`
  (params (PlayRate :type "Float (single-precision)" :default 1.0))
  (bind _v_currectloc (`self.v_CurrectLoc`))
  (`TimelineComponent.SetPlayRate` (`self.TL_Launch`) PlayRate)
  (`self.SetActorHiddenInGame` false)
  (`PaperSpriteComponent.SetSpriteColor` (`self.PaperSprite`) (struct :`R` 1.0 :`G` 1.0 :`B` 1.0 :`A` 1.0))
  (bind (_direction _alpha) (`Timeline|TL_Launch` :!via `PlayFromStart`)
    (:`Update`
      (`self.K2_SetActorLocation` (`KismetMathLibrary.VLerp` _v_currectloc (+ _v_currectloc (0.0 0.0 400.0)) _alpha)))
    (:`Finished`
      (`self.StartLifeTime`))))

(event `ActivateCanOverlapped`
  (set `self.b_CanBeOverlapped` true)
  (`self.SetActorEnableCollision` true))

(event `StartLifeTime`
  (bind (_direction _alpha) (`Timeline|TL_LifeTime` :!via `PlayFromStart`)
    (:`Update`
      (`PaperSpriteComponent.SetSpriteColor` (`self.PaperSprite`) (`KismetMathLibrary.MakeColor` 1.0 1.0 1.0 _alpha)))
    (:`Finished`
      (`self.ForceToPool`))))

(fn `OnOverlapEvent`
  (`/Game/_BottomlessPit/Blueprint/FunctionLibrary/BFL_GameFeels.StartVFXTransform` (`KismetMathLibrary.MakeTransform` (+ (`self.K2_GetActorLocation` (`GameplayStatics.GetPlayerCharacter` 0)) (`KismetMathLibrary.MakeVector` (`KismetMathLibrary.RandomFloatInRange` -120.0 120.0) 0.0 -150.0))) (`self.Fn_CurrentWeaponName`)))

(fn `UserConstructionScript`)