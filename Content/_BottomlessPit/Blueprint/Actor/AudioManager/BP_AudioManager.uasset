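; BP_AudioManager is an audio manager actor that plays 2D sound effects, gameplay music and main menu music through interface-style events.
; Effects load asynchronously by row name from a data table and are cached in a map for replay.
; Each music track's audio component is created on first request, then reused for fade-in and fade-out.
; MuteBgm silences the BGM sound class through a sound mix override.
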(event `self.ReceiveBeginPlay`)

(event `/Game/_BottomlessPit/Blueprint/Interface/BPI_Actor.I_ActivateSFX`
  (params (SFXName :type Name))
  ; SFX
  (`self.ActivateVFX` SFXName))

(event `ActivateVFX`
  (params (RowName :type Name))
  (bind (_value _returnvalue) (`BlueprintMapLibrary.Map_Find` (`self.ChachedSFX`) RowName))
  ; SFX
  (if _returnvalue
    (`GameplayStatics.PlaySound2D` (`.Sound` (break `SFXDataResolved` _value)) 1.0 1.0 0.0 null null)
    (else
      (bind (_rowname _sfx) (`Util_BpAsyncSFX.LoadSFXDataRowAsync` (`self.DT_SFX`) RowName)
        (:`OnCompleted`
          (`BlueprintMapLibrary.Map_Add` (`self.ChachedSFX`) RowName _sfx)
          (`GameplayStatics.PlaySound2D` (`.Sound` (break `SFXDataResolved` _sfx)) 1.0 1.0 0.0 null null))))))

(event `/Game/_BottomlessPit/Blueprint/Interface/BPI_Actor.I_StartBgm`
  ; BGM Gameplay
  (`/Engine/EditorBlueprintResources/StandardMacros.IsValid` (`self.BGM`)
    (:`Is Valid`
      (`AudioComponent.FadeIn` (`self.BGM`) 1.0 1.0 0.0 "Linear"))
    (:`Is Not Valid`
      (bind (_rowname _sfx) (`Util_BpAsyncSFX.LoadSFXDataRowAsync` (`self.DT_SFX`) "Bgm")
        (:`OnCompleted`
          (bind _returnvalue (`GameplayStatics.CreateSound2D` (`.Sound` (break `SFXDataResolved` _sfx)) 1.0 1.0 0.0 null))
          (bind _output_get (set `self.BGM` _returnvalue))
          (`AudioComponent.FadeIn` _output_get 2.0 1.0 0.0 "Linear"))))))

(event `/Game/_BottomlessPit/Blueprint/Interface/BPI_Actor.I_StopBgm`
  ; BGM Gameplay
  (`/Engine/EditorBlueprintResources/StandardMacros.IsValid` (`self.BGM`)
    (:`Is Valid`
      (`AudioComponent.FadeOut` (`self.BGM`) 0.5 0.0 "Linear"))
    (:`Is Not Valid`
      (bind (_rowname _sfx) (`Util_BpAsyncSFX.LoadSFXDataRowAsync` (`self.DT_SFX`) "Bgm")
        (:`OnCompleted`
          (bind _returnvalue (`GameplayStatics.CreateSound2D` (`.Sound` (break `SFXDataResolved` _sfx)) 1.0 1.0 0.0 null))
          (bind _output_get (set `self.BGM` _returnvalue))
          (`AudioComponent.FadeOut` _output_get 2.5 0.0 "Linear"))))))

(event `/Game/_BottomlessPit/Blueprint/Interface/BPI_Actor.I_StartMainMenu`
  ; BGM MainMenu
  (`/Engine/EditorBlueprintResources/StandardMacros.IsValid` (`self.BgmMainMenu`)
    (:`Is Valid`
      (`AudioComponent.FadeIn` (`self.BgmMainMenu`) 1.0 1.0 0.0 "Linear"))
    (:`Is Not Valid`
      (bind (_rowname _sfx) (`Util_BpAsyncSFX.LoadSFXDataRowAsync` (`self.DT_SFX`) "BgmMainMenu")
        (:`OnCompleted`
          (bind _returnvalue (`GameplayStatics.CreateSound2D` (`.Sound` (break `SFXDataResolved` _sfx)) 1.0 1.0 0.0 null))
          (bind _output_get (set `self.BgmMainMenu` _returnvalue))
          (`AudioComponent.FadeIn` _output_get 2.0 1.0 0.0 "Linear"))))))

(event `/Game/_BottomlessPit/Blueprint/Interface/BPI_Actor.I_StopMainMenu`
  ; BGM MainMenu
  (`/Engine/EditorBlueprintResources/StandardMacros.IsValid` (`self.BgmMainMenu`)
    (:`Is Valid`
      (`AudioComponent.FadeOut` (`self.BgmMainMenu`) 0.5 0.0 "Linear"))
    (:`Is Not Valid`
      (bind (_rowname _sfx) (`Util_BpAsyncSFX.LoadSFXDataRowAsync` (`self.DT_SFX`) "BgmMainMenu")
        (:`OnCompleted`
          (bind _returnvalue (`GameplayStatics.CreateSound2D` (`.Sound` (break `SFXDataResolved` _sfx)) 1.0 1.0 0.0 null))
          (bind _output_get (set `self.BgmMainMenu` _returnvalue))
          (`AudioComponent.FadeOut` _output_get 2.5 0.0 "Linear"))))))

(event `MuteBgm`
  (bind _sm_bgm (`self.SM_BGM`))
  (`GameplayStatics.PushSoundMixModifier` _sm_bgm)
  (`GameplayStatics.SetSoundMixClassOverride` _sm_bgm "/Game/_BottomlessPit/Blueprint/Actor/AudioManager/SoundClass/SC_BGM.SC_BGM" 0.0))

(fn `UserConstructionScript`)