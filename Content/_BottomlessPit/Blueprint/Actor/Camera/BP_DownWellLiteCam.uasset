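; Orthographic follow camera for the player character, registering itself with the player at BeginPlay and reacting to camera interface events.
; First input eases the follow lerp speed down from its fast starting value.
; Death focuses on the player and narrows the ortho width before triggering the game-over sequence, while restart reverses the zoom and cancels focus.
; Slam-down widens or restores the ortho width through a timeline played forward or backward.
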(event `self.ReceiveBeginPlay`
  (bind _returnvalue (`GameplayStatics.GetPlayerCharacter` 0))
  (set `self.FollowTarget` _returnvalue)
  (message `/Game/_BottomlessPit/Blueprint/Interface/BPI_Player.I_P1_Blp_RegisterCamera` _returnvalue self)
  (set `self.FollowLerpSpeed` 60.0)
  (set `self.f_OriginalOrthoWidth` (`self.OrthoWidth`)))

(event `SetCamPlay`
  (bind (_direction _alpha) (`Timeline|LerpCamSpeed` :!via `PlayFromStart`)
    (:`Update`
      (set `self.FollowLerpSpeed` (`KismetMathLibrary.Lerp` 60.0 6.0 _alpha)))))

(event `OnDeathCamera Lerp`
  (bind _f_originalorthowidth (`self.f_OriginalOrthoWidth`))
  (bind (_direction _alpha) (`Timeline|LerpCamDead` :!via `PlayFromStart` :!label _label)
    (:`Update`
      (set `self.OrthoWidth` (`KismetMathLibrary.Lerp` _f_originalorthowidth (- _f_originalorthowidth 750.0) _alpha)))
    (:`Finished`
      (if (`|EnumEquality` _direction "Forward")
        (message `/Game/_BottomlessPit/Blueprint/Interface/BPI_Player.I_P1_PlayGameOverSequence` (`GameplayStatics.GetPlayerCharacter` 0))
        (else
          (set `self.FollowLerpSpeed` 60.0))))))

(event `OnRestartCameraLerp`
  (goto _label :!via `ReverseFromEnd`))

(event `/Game/_BottomlessPit/Blueprint/Interface/BPI_Actor.I_Cam_OnFirstInput`
  (`self.SetCamPlay`))

(event `/Game/_BottomlessPit/Blueprint/Interface/BPI_Actor.I_Cam_OnDead`
  (`self.FocusOnActor` (`self.FollowTarget`) 40.0)
  (`self.OnDeathCamera Lerp`))

(event `/Game/_BottomlessPit/Blueprint/Interface/BPI_Actor.I_Cam_OnRestart`
  (`self.OnRestartCameraLerp`)
  (`self.CancelFocus`))

(event `/Game/_BottomlessPit/Blueprint/Interface/BPI_Actor.I_Cam_OnSlamDown`
  (params (`Forward?` :type Boolean))
  (`self.SlamDown` `Forward?`))

(event `SlamDown`
  (params (`Forward?` :type Boolean))
  (bind _returnvalue (`KismetMathLibrary.SelectFloat` 2.0 2.5 `Forward?`))
  (bind _f_originalorthowidth (`self.f_OriginalOrthoWidth`))
  (if `Forward?`
    (`TimelineComponent.SetPlayRate` (`self.TL_SlamDown`) _returnvalue)
    (bind (_direction _alpha) (`Timeline|TL_SlamDown` :!via `PlayFromStart` :!label _label_2)
      (:`Update`
        (set `self.OrthoWidth` (`KismetMathLibrary.Lerp` _f_originalorthowidth (+ _f_originalorthowidth 300.0) _alpha))))
    (else
      (`TimelineComponent.SetPlayRate` (`self.TL_SlamDown`) _returnvalue)
      (goto _label_2 :!via `ReverseFromEnd`))))

(fn `UserConstructionScript`)