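; BP_LaneLevelGenerator is a level actor that controls the lane level's platform spawning, switched on and off through interface events.
; On BeginPlay it registers itself with the player pawn, and it stores a camera reference when one is sent.
; Activation enables spawning, turns off Z looping and recenters world Z.
; Deactivation pauses and flushes, including walls, and disables wall blockers; the generation logic itself is not in this graph.
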(event `self.ReceiveBeginPlay`
  (bind _output_get (set `self.PlayerRef` (`GameplayStatics.GetPlayerPawn` 0)))
  (message `/Game/_BottomlessPit/Blueprint/Interface/BPI_Player.I_P1_Blp_RegisterLaneLevel` _output_get self))

(event `/Game/_BottomlessPit/Blueprint/Interface/BPI_Actor.I_Blp_ActivatePlatform`
  (params (`True?` :type Boolean))
  (bind _output_get (set `self.bSpawnPlatforms` `True?`))
  (bind _output_get_2 (set `self.bUseZLoop` (not _output_get)))
  (if (not _output_get_2)
    (`self.RecenterWorldZ` true)))

(event `/Game/_BottomlessPit/Blueprint/Interface/BPI_Actor.I_Blp_DeactivatePlatform`
  (params (`True?` :type Boolean))
  (`self.PauseAndFlush` `True?` `True?`))

(event `/Game/_BottomlessPit/Blueprint/Interface/BPI_Actor.I_Blp_RegisterCamera`
  (params (RefIn :type "Actor Object Reference"))
  (set `self.CameraActor` RefIn))

(fn `UserConstructionScript`)