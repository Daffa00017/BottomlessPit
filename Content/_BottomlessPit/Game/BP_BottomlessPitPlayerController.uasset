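; Player controller for Bottomless Pit that runs menu, pause, restart and quit-confirm flow and takes motion input from an Arduino.
; On BeginPlay it spawns BP_DownWellLiteCam above the player as view target and relays first-input, death and restart messages to it.
; Inputs branch on game state and readiness flags, messaging character and HUD through interfaces.
; A looping timer polls the serial port, parsing comma-separated X/Y readings into ApplyArduinoAccelVector.
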(event `self.ReceiveBeginPlay`
  (bind _returnvalue (`|SpawnActorFromClass` "/Game/_BottomlessPit/Blueprint/Actor/Camera/BP_DownWellLiteCam.BP_DownWellLiteCam_C" (`KismetMathLibrary.MakeTransform` (+ (`self.K2_GetActorLocation` (`GameplayStatics.GetPlayerCharacter` 0)) (0.0 0.0 1550.0))) "Undefined" "MultiplyWithRoot" null null))
  (bind _output_get (set `self.Reff_CameraManager` _returnvalue))
  (`CPP_CameraManager.AdoptAsViewTarget` _output_get 0.25)
  (`self.SetViewTargetWithBlend` _output_get)
  (`self.RegisterArduino`))

(event `/Game/_BottomlessPit/Blueprint/Interface/BPI_PlayerController.I_Pc_OnFirstInput`
  (message `/Game/_BottomlessPit/Blueprint/Interface/BPI_Actor.I_Cam_OnFirstInput` (`self.Reff_CameraManager`)))

(event `/Game/_BottomlessPit/Blueprint/Interface/BPI_PlayerController.I_Pc_OnDead`
  (params (`Dead?` :type Boolean))
  (bind _output_get (set `self.IsPlayerDead` `Dead?`))
  (if _output_get
    (message `/Game/_BottomlessPit/Blueprint/Interface/BPI_Actor.I_Cam_OnDead` (`self.Reff_CameraManager`))))

(event `/Game/_BottomlessPit/Blueprint/Interface/BPI_PlayerController.I_Pc_OnRestart`
  (message `/Game/_BottomlessPit/Blueprint/Interface/BPI_Actor.I_Cam_OnRestart` (`self.Reff_CameraManager`)))

(event `self.OnEscapeInput`
  (if (`self.IsInMainMenu`)
    (if (`self.b_ReadyToConfirmQuit`)
      (if (`self.ConfirmToExit`)
        (set `self.ConfirmToExit` false)
        (message `/Game/_BottomlessPit/Blueprint/Interface/BPI_HUDAndUI.I_UI_ConfirmOnExit` (`self.GetHUD` (`GameplayStatics.GetPlayerController` 0)) false)
        (set `self.b_ReadyToConfirmQuit` false)
        (`/Game/_BottomlessPit/Blueprint/FunctionLibrary/BFL_GameFeels.StartSFX` "Select")
        (else
          (set `self.ConfirmToExit` true)
          (message `/Game/_BottomlessPit/Blueprint/Interface/BPI_HUDAndUI.I_UI_ConfirmOnExit` (`self.GetHUD` (`GameplayStatics.GetPlayerController` 0)) true)
          (set `self.b_ReadyToConfirmQuit` false)
          (`/Game/_BottomlessPit/Blueprint/FunctionLibrary/BFL_GameFeels.StartSFX` "Select")))
      (else
        (`KismetSystemLibrary.PrintString` "GakValid")))
    (else
      (`self.PauseGame`))))

(event `ForcedFirstInput`
  (bind _isdead_ (message `/Game/_BottomlessPit/Blueprint/Interface/BPI_Player.I_P1_IsPlayerDead` (`GameplayStatics.GetPlayerCharacter` 0) :!label _label))
  (if _isdead_
    (if (`self.b_ReadyToRestart`)
      (`KismetSystemLibrary.PrintString` "Restart")
      (set `self.IsInMainMenu` true)
      (message `/Game/_BottomlessPit/Blueprint/Interface/BPI_Player.I_P1_ReadyToRestart` (`GameplayStatics.GetPlayerCharacter` 0) false)
      (message `/Game/_BottomlessPit/Blueprint/Interface/BPI_HUDAndUI.I_UI_Restart` (`self.GetHUD` (`GameplayStatics.GetPlayerController` 0)))
      (message `/Game/_BottomlessPit/Blueprint/Interface/BPI_Player.I_P1_PlayerOnRestart` (`GameplayStatics.GetPlayerCharacter` 0))
      (`/Game/_BottomlessPit/Blueprint/FunctionLibrary/BFL_GameFeels.StartSFX` "Select"))
    (elif (`self.ConfirmToExit`)
      _
      (elif (`self.b_ReadyToMainMenu`)
        (if (`self.IsInMainMenu`)
          (set `self.IsInMainMenu` false)
          (message `/Game/_BottomlessPit/Blueprint/Interface/BPI_Player.I_P1_PlayerOnFirstInput` (`GameplayStatics.GetPlayerCharacter` 0))
          (`/Game/_BottomlessPit/Blueprint/FunctionLibrary/BFL_GameFeels.StartBgm`)
          (`/Game/_BottomlessPit/Blueprint/FunctionLibrary/BFL_GameFeels.StopBgmMainMenu`))))))

(event `self.OnFirstInput`
  (goto _label))

(event `PauseGame`
  (if (`GameplayStatics.IsGamePaused`)
    (`GameplayStatics.SetGamePaused` false)
    (message `/Game/_BottomlessPit/Blueprint/Interface/BPI_HUDAndUI.I_UI_OnPause` (`self.GetHUD` (`GameplayStatics.GetPlayerController` 0)) false)
    (`/Game/_BottomlessPit/Blueprint/FunctionLibrary/BFL_GameFeels.StartSFX` "Select")
    (else
      (`GameplayStatics.SetGamePaused` true)
      (message `/Game/_BottomlessPit/Blueprint/Interface/BPI_HUDAndUI.I_UI_OnPause` (`self.GetHUD` (`GameplayStatics.GetPlayerController` 0)) true)
      (`/Game/_BottomlessPit/Blueprint/FunctionLibrary/BFL_GameFeels.StartSFX` "Select"))))

(event `/Game/_BottomlessPit/Blueprint/Interface/BPI_PlayerController.I_Pc_ReadyToRestart`
  (params (`Ready?` :type Boolean))
  (set `self.b_ReadyToRestart` `Ready?`))

(event `/Game/_BottomlessPit/Blueprint/Interface/BPI_PlayerController.I_Pc_ReadyToMainMenu`
  (params (`Ready?` :type Boolean))
  (set `self.b_ReadyToMainMenu` `Ready?`))

(event `self.OnQuitGame`
  (`KismetSystemLibrary.QuitGame` self "Quit"))

(event `/Game/_BottomlessPit/Blueprint/Interface/BPI_PlayerController.I_Pc_ReadyToConfirmQuit`
  (params (`Ready?` :type Boolean))
  (set `self.b_ReadyToConfirmQuit` `Ready?`))

(event `RegisterArduino`
  (bind (_bopened _returnvalue) (`SerialCom.OpenComPort` 7 115200))
  (`/Engine/EditorBlueprintResources/StandardMacros.IsValid` _returnvalue
    (:`Is Valid`
      (if (`SerialCom.IsOpened` _returnvalue)
        (bind _output_get (set `self.SerialPortRef` _returnvalue))
        (`SerialCom.Flush` _output_get)
        (`SerialCom.Println` _returnvalue "We are connected ")
        (`KismetSystemLibrary.PrintString` "PortInit")
        (`KismetSystemLibrary.K2_SetTimerDelegate` (`|CreateDelegate` :!event `ArduinoInput`) 0.01 true)
        (else
          (`KismetSystemLibrary.PrintString` "PortIsNotConnected"))))))

(event `ArduinoInput`
  (bind (_bsuccess _returnvalue) (`SerialCom.ReadString` (`self.SerialPortRef`)))
  (if _bsuccess
    (bind _returnvalue_2 (`KismetStringLibrary.ParseIntoArray` _returnvalue ","))
    (if (>= (`KismetArrayLibrary.Array_Length` _returnvalue_2) 2)
      (`self.ApplyArduinoAccelVector` (`KismetMathLibrary.MakeVector2D` (* (`KismetStringLibrary.Conv_StringToDouble` (`|GetArrayItem` _returnvalue_2)) 1.0) (* (`KismetStringLibrary.Conv_StringToDouble` (`|GetArrayItem` _returnvalue_2 1)) 1.0))))))

(event `self.ReceiveEndPlay`
  (params (EndPlayReason :type "EEndPlayReason Enum" :default "Destroyed"))
  (bind _serialportref (`self.SerialPortRef`))
  (`/Engine/EditorBlueprintResources/StandardMacros.IsValid` _serialportref
    (:`Is Valid`
      (`SerialCom.Close` _serialportref))))

(fn `UserConstructionScript`)