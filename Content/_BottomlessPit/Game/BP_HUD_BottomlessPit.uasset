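; BP_HUD_BottomlessPit is the HUD Blueprint for the Bottomless Pit game, acting as a relay between gameplay and the gameplay UI widget.
; It receives UI interface events for game flow (play, pause, restart, exit confirm), ammo, health and death, score, and combo.
; Each event forwards its values unchanged as the matching interface message to WBGameplayUIReference, with no logic of its own.
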(event `/Game/_BottomlessPit/Blueprint/Interface/BPI_HUDAndUI.I_UI_OnPlay`
  ;[1 1 1 0.6706] Game
  (message `/Game/_BottomlessPit/Blueprint/Interface/BPI_HUDAndUI.I_UI_OnPlay` (`self.WB_GameplayUIReference`)))

(event `/Game/_BottomlessPit/Blueprint/Interface/BPI_HUDAndUI.I_UI_Restart`
  ;[1 1 1 0.6706] Game
  (message `/Game/_BottomlessPit/Blueprint/Interface/BPI_HUDAndUI.I_UI_Restart` (`self.WB_GameplayUIReference`)))

(event `/Game/_BottomlessPit/Blueprint/Interface/BPI_HUDAndUI.I_UI_ConfirmOnExit`
  (params (`True?` :type Boolean))
  ;[1 1 1 0.6706] Game
  (message `/Game/_BottomlessPit/Blueprint/Interface/BPI_HUDAndUI.I_UI_ConfirmOnExit` (`self.WB_GameplayUIReference`) `True?`))

(event `/Game/_BottomlessPit/Blueprint/Interface/BPI_HUDAndUI.I_UI_OnPause`
  (params (`IsPause?` :type Boolean))
  ;[1 1 1 0.6706] Game
  (message `/Game/_BottomlessPit/Blueprint/Interface/BPI_HUDAndUI.I_UI_OnPause` (`self.WB_GameplayUIReference`) `IsPause?`))

(event `/Game/_BottomlessPit/Blueprint/Interface/BPI_HUDAndUI.I_UI_Blp_OnCurrentAmmoChange`
  (params (CurrentAmmoIn :type Integer))
  ;[0.2086 0.8388 0.9047 0.502] Ammo
  (message `/Game/_BottomlessPit/Blueprint/Interface/BPI_HUDAndUI.I_UI_Blp_OnCurrentAmmoChange` (`self.WB_GameplayUIReference`) CurrentAmmoIn))

(event `/Game/_BottomlessPit/Blueprint/Interface/BPI_HUDAndUI.I_UI_Blp_OnMaxAmmoChange`
  (params (MaxAmmoIn :type Integer))
  ;[0.2086 0.8388 0.9047 0.502] Ammo
  (message `/Game/_BottomlessPit/Blueprint/Interface/BPI_HUDAndUI.I_UI_Blp_OnMaxAmmoChange` (`self.WB_GameplayUIReference`) MaxAmmoIn))

(event `/Game/_BottomlessPit/Blueprint/Interface/BPI_HUDAndUI.I_UI_Blp_OnAmmoFill`
  (params (CurrentAmmoIn :type Integer))
  ;[0.2086 0.8388 0.9047 0.502] Ammo
  (message `/Game/_BottomlessPit/Blueprint/Interface/BPI_HUDAndUI.I_UI_Blp_OnAmmoFill` (`self.WB_GameplayUIReference`) CurrentAmmoIn))

(event `/Game/_BottomlessPit/Blueprint/Interface/BPI_HUDAndUI.I_UI_OnMaxHealthChange`
  (params (MaxHealthIn :type "Float (double-precision)"))
  ;[0 1 0.3813 0.502] Health
  (message `/Game/_BottomlessPit/Blueprint/Interface/BPI_HUDAndUI.I_UI_OnMaxHealthChange` (`self.WB_GameplayUIReference`) MaxHealthIn))

(event `/Game/_BottomlessPit/Blueprint/Interface/BPI_HUDAndUI.I_UI_OnHealthChange`
  (params (CurrentHealthIn :type "Float (double-precision)"))
  ;[0 1 0.3813 0.502] Health
  (message `/Game/_BottomlessPit/Blueprint/Interface/BPI_HUDAndUI.I_UI_OnHealthChange` (`self.WB_GameplayUIReference`) CurrentHealthIn))

(event `/Game/_BottomlessPit/Blueprint/Interface/BPI_HUDAndUI.I_UI_OnDeath`
  ;[0 1 0.3813 0.502] Health
  (message `/Game/_BottomlessPit/Blueprint/Interface/BPI_HUDAndUI.I_UI_OnDeath` (`self.WB_GameplayUIReference`)))

(event `/Game/_BottomlessPit/Blueprint/Interface/BPI_HUDAndUI.I_UI_Blp_UpdateScore`
  (params (NewScoreIn :type "Float (double-precision)"))
  ;[0.227 0.7305 0.2346 0.502] Score
  (message `/Game/_BottomlessPit/Blueprint/Interface/BPI_HUDAndUI.I_UI_Blp_UpdateScore` (`self.WB_GameplayUIReference`) NewScoreIn))

(event `/Game/_BottomlessPit/Blueprint/Interface/BPI_HUDAndUI.I_UI_Blp_ShowComboUI`
  ;[0.15 0.1466 0.05454 0.5] Combo
  (message `/Game/_BottomlessPit/Blueprint/Interface/BPI_HUDAndUI.I_UI_Blp_ShowComboUI` (`self.WB_GameplayUIReference`)))

(event `/Game/_BottomlessPit/Blueprint/Interface/BPI_HUDAndUI.I_UI_Blp_HideComboUI`
  ;[0.15 0.1466 0.05454 0.5] Combo
  (message `/Game/_BottomlessPit/Blueprint/Interface/BPI_HUDAndUI.I_UI_Blp_HideComboUI` (`self.WB_GameplayUIReference`)))

(event `/Game/_BottomlessPit/Blueprint/Interface/BPI_HUDAndUI.I_UI_Blp_UpdateComboTimer`
  (params (PercentageIn :type "Float (double-precision)"))
  ;[0.15 0.1466 0.05454 0.5] Combo
  (message `/Game/_BottomlessPit/Blueprint/Interface/BPI_HUDAndUI.I_UI_Blp_UpdateComboTimer` (`self.WB_GameplayUIReference`) PercentageIn))

(event `/Game/_BottomlessPit/Blueprint/Interface/BPI_HUDAndUI.I_UI_Blp_UpdateCombo`
  (params (ComboIn :type "Float (double-precision)"))
  ;[0.15 0.1466 0.05454 0.5] Combo
  (message `/Game/_BottomlessPit/Blueprint/Interface/BPI_HUDAndUI.I_UI_Blp_UpdateCombo` (`self.WB_GameplayUIReference`) ComboIn))

(event `/Game/_BottomlessPit/Blueprint/Interface/BPI_HUDAndUI.I_UI_Blp_UpdateMultiplerCombo`
  (params (MultIn :type "Float (double-precision)"))
  ;[0.15 0.1466 0.05454 0.5] Combo
  (message `/Game/_BottomlessPit/Blueprint/Interface/BPI_HUDAndUI.I_UI_Blp_UpdateMultiplerCombo` (`self.WB_GameplayUIReference`) MultIn))

(fn `UserConstructionScript`)